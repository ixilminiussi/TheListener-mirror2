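; BP_Tape is an interactive tape prop whose two wheels spin while it is switched on.
; Interacting flips the IsOn flag.
; While on, Tick rotates Weel and Weel1 in pitch by SpinSpeed scaled by delta time, with the second wheel's speed multiplied by Ratio.
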(event EventBeginPlay)

(event Collision|EventActorBeginOverlap
  (params (OtherActor :type Actor%20Object%20Reference)))

(event EventTick
  (params (DeltaSeconds :type Float%20%28single-precision%29))
  (bind _spinspeed (Variables|Default|GetSpinSpeed))
  (bind _returnvalue (* DeltaSeconds _spinspeed))
  (if (Variables|Default|GetIsOn)
    (Transformation|AddLocalRotation (Variables|Default|Getweel) (Math|Rotator|MakeRotator 0.0 _returnvalue 0.0) false false)
    (Transformation|AddLocalRotation (Variables|Default|Getweel1) (Math|Rotator|MakeRotator 0.0 (* _returnvalue (Variables|Default|GetRatio)) 0.0) false false)))

(event EventOnInteract
  (Variables|Default|SetIsOn (not (Variables|Default|GetIsOn))))

(fn ConstructionScript)