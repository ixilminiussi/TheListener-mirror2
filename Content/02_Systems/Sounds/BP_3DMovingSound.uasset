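; Actor that plays a Wwise sound from an Ak component that can travel along a spline.
; PlaySound posts SoundToPlay, optionally at BeginPlay via PlayAtBeginning, and StopSound stops it.
; MoveObject runs a Timeline scaled by TimeToComplete, lerping distance over the spline length to position the emitter.
; Spline values are read in local space but applied as world transforms, with rotation always sampled at the spline start.
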(event Custom|PlaySound
  (bind _ak (Variables|Default|GetAk))
  (bind _output_get (Variables|/Script/AkAudio.AkGameObject|SetAkAudioEvent _ak (Variables|Default|GetSoundToPlay)))
  (Class|AkGameObject|PostAkEvent _ak _output_get))

(event Custom|StopSound
  (Class|AkGameObject|Stop (Variables|Default|GetAk)))

(event Custom|MoveObject
  (bind _spline (Variables|Default|GetSpline))
  (Components|Timeline|SetPlayRate (Variables|Default|GetTimeline) (/ 1.0 (Variables|Default|GetTimeToComplete)))
  (bind _move_track (Timeline|Timeline Play)
    (:Update
      (Transformation|SetWorldLocationAndRotation (Variables|Default|GetAk) (Spline|GetLocationatDistanceAlongSpline _spline (Math|Float|Lerp 0.0 (Spline|GetSplineLength _spline) _move_track) "Local") (Spline|GetRotationatDistanceAlongSpline _spline 0.0 "Local") false false))))

(event EventBeginPlay
  (bind _ak (Variables|Default|GetAk))
  (if (Variables|Default|GetPlayAtBeginning?)
    (bind _output_get (Variables|/Script/AkAudio.AkGameObject|SetAkAudioEvent _ak (Variables|Default|GetSoundToPlay)))
    (Class|AkGameObject|PostAkEvent _ak _output_get)))

(fn ConstructionScript)