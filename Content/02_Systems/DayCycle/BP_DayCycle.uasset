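; Day cycle actor that animates the level's sun by rotating a Directional Light over time.
; On BeginPlay it finds the light with GetActorOfClass and sets its pitch to a configurable start angle, keeping yaw and roll.
; Tick raises the pitch at a frame-rate-independent speed and records the current angle.
; Movement is one-way and stops once the pitch passes the angle cap, with no looping.
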(event EventBeginPlay
  (bind _returnvalue (Actor|GetActorOfClass "/Script/Engine.DirectionalLight"))
  (bind _output_get (Variables|Default|SetSun _returnvalue))
  (Transformation|SetActorRotation _output_get (Math|Rotator|MakeRotator (.roll (Transformation|GetActorRotation _output_get)) (Variables|Default|GetStartSunAngle) (.yaw (Transformation|GetActorRotation _output_get)))))

(event EventTick
  (params (DeltaSeconds :type Float%20%28single-precision%29))
  (bind _sun (Variables|Default|GetSun)
    (:then
      (if (<= (.pitch (Transformation|GetActorRotation _sun)) (Variables|Default|GetAngleCap))
        (Transformation|SetActorRotation _sun (Math|Rotator|MakeRotator (.roll (Transformation|GetActorRotation _sun)) (+ (.pitch (Transformation|GetActorRotation _sun)) (* DeltaSeconds (Variables|Default|GetSunSpeed))) (.yaw (Transformation|GetActorRotation _sun))))
        (Variables|Default|SetCurrentSunAngle (.pitch (Transformation|GetActorRotation _sun)))))
    (:else)))

(fn ConstructionScript)