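; BP_CableManager is a manager actor that sizes the level's cable components and sways them with randomized wind.
; On BeginPlay it gathers CableComponents from StaticMeshActors, setting each length to a percentage of its endpoint distance and applying an initial force.
; A looping timer then rerolls intensity within a range and pushes one shared force to all cached cables.
; Force direction uses Ultra Dynamic Weather's WindDirection as rotator pitch, not yaw.
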(event Custom|RefreshWind
  (CallFunction|UpdateWindIntensity true))

(event EventBeginPlay
  (CallFunction|RefreshCableVariable)
  (Utilities|Time|SetTimerbyEvent (delegate Custom|RefreshWind) (Variables|Default|GetIntervalBetweenUpdate) true))

(event Collision|EventActorBeginOverlap
  (params (OtherActor :type Actor%20Object%20Reference)))

(event EventTick
  (params (DeltaSeconds :type Float%20%28single-precision%29)))

(fn ConstructionScript)

(fn RefreshCableVariable
  (bind _returnvalue (Actor|GetActorOfClass "/Game/UltraDynamicSky/Blueprints/Ultra_Dynamic_Weather.Ultra_Dynamic_Weather_C"))
  (Variables|Default|SetWeatherBlueprint _returnvalue)
  (CallFunction|UpdateWindIntensity false)
  (bind _outactors (Actor|GetAllActorsOfClass "/Script/Engine.StaticMeshActor"))
  (Utilities|Array|Clear (Variables|Default|GetCables))
  (for _array_element _outactors
    (for (_array_element_2 _array_index) (Actor|GetComponentsByClass _array_element "/Script/CableComponent.CableComponent")
      (Utilities|Array|Add (Variables|Default|GetCables) _array_element_2)
      (CallFunction|SetCableVariable _array_element_2)
      (if (== _array_index 0)
        _))))

(fn SetCableVariable
  (params (Component :type Cable%20Component%20Object%20Reference))
  (Variables|/Script/CableComponent.CableComponent|SetCableLength Component (* (CallFunction|GetCableDistance Component) (Variables|Default|GetCableDistancePercentage)))
  (Variables|/Script/CableComponent.CableComponent|SetCableForce Component (Variables|Default|GetCableForce)))

(fn GetCableDistance
  (params (Cable :type Cable%20Component%20Object%20Reference))
  (bind _returnvalue (Class|CableComponent|GetAttachedActor Cable))
  (Utilities|IsValid _returnvalue
    (:Is%20Valid
      (LocalVariables|SetEndPointLocation (Transformation|GetActorLocation _returnvalue)))
    (:Is%20Not%20Valid
      (LocalVariables|SetEndPointLocation (Transformation|GetWorldLocation Cable))))
  (return (Math|Vector|Distance(Vector) (Transformation|GetWorldLocation Cable) (+ (Variables|/Script/CableComponent.CableComponent|GetEndLocation Cable) (LocalVariables|GetEndPointLocation)))))

(fn UpdateWindIntensity
  (params (Apply :type Boolean))
  (bind _windintensity (Variables|Default|GetWindIntensity))
  (Variables|Default|SetCurrentWindIntensity (Math|Random|RandomFloatinRange (.x _windintensity) (.y _windintensity)))
  (CallFunction|GetCableForce)
  (if Apply
    (for _array_element (Variables|Default|GetCables)
      (Variables|/Script/CableComponent.CableComponent|SetCableForce _array_element (Variables|Default|GetCableForce)))))

(fn GetCableForce
  (bind _weatherblueprint (Variables|Default|GetWeatherBlueprint))
  (Utilities|IsValid _weatherblueprint
    (:Is%20Valid
      (LocalVariables|SetWindDir (Variables|/Game/UltraDynamicSky/Blueprints/Ultra_Dynamic_Weather.Ultra_Dynamic_Weather_C|GetWind%20Direction _weatherblueprint)))
    (:Is%20Not%20Valid
      _))
  (Variables|Default|SetCableForce (* (Math|Vector|GetForwardVector (Math|Rotator|MakeRotator 0.0 (LocalVariables|GetWindDir) 0.0)) (Variables|Default|GetCurrentWindIntensity))))