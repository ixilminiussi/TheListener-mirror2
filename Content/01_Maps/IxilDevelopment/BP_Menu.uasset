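; BP_Menu is an actor that hosts a menu through its Widget component and relays up/down navigation input to it.
; On BeginPlay it sets the first player controller to Game and UI input mode, focusing the component's user widget.
; The IA_Up and IA_Down input actions cast that widget to WBP_Menu and call GoUp or GoDown.
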(event Input|EnhancedActionEvents|EnhancedInputActionIA_Up
  (params (ActionValue :type Boolean) (ElapsedSeconds :type Float%20%28double-precision%29) (TriggeredSeconds :type Float%20%28double-precision%29) (InputAction :type Input%20Action%20Object%20Reference :default "/Game/01_Maps/IxilDevelopment/IA_Up.IA_Up"))
  (bind _aswbp_menu (Utilities|Casting|CastToWBP_Menu (UserInterface|GetWidget (Variables|Default|GetWidget))))
  (Default|GoUp _aswbp_menu))

(event Input|EnhancedActionEvents|EnhancedInputActionIA_Down
  (params (ActionValue :type Boolean) (ElapsedSeconds :type Float%20%28double-precision%29) (TriggeredSeconds :type Float%20%28double-precision%29) (InputAction :type Input%20Action%20Object%20Reference :default "/Game/01_Maps/IxilDevelopment/IA_Down.IA_Down"))
  (bind _aswbp_menu (Utilities|Casting|CastToWBP_Menu (UserInterface|GetWidget (Variables|Default|GetWidget))))
  (Default|GoDown _aswbp_menu))

(event EventBeginPlay
  (Input|SetInputModeGameandUI (Game|GetPlayerController 0) (UserInterface|GetUserWidgetObject (Variables|Default|GetWidget)) "LockOnCapture" false false))

(event Collision|EventActorBeginOverlap
  (params (OtherActor :type Actor%20Object%20Reference)))

(event EventTick
  (params (DeltaSeconds :type Float%20%28single-precision%29)))

(fn ConstructionScript)