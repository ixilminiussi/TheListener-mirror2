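; BP_LukaHUD is the in-game HUD that handles cinematic black bars and the pause and settings menus.
; It creates the black bars widget on BeginPlay, plays its FadeIn forward or reversed for cinematics, and exposes that animation's length.
; Pausing adds a game layout at very high Z-order and pushes menus onto it; closing settings re-pushes the previous menu class before removing the settings widget.
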(event Custom|EndCinematic
  (bind _blackbars (Variables|Default|GetBlackBars))
  ;[0.02922 0.15 0.0212 0.5] Leo's Black Bar
  (Utilities|IsValid _blackbars
    (:Is%20Valid
      (UserInterface|Animation|PlayAnimation _blackbars (Variables|/Game/07_UI/InGame/General/WBP_BlackBars.WBP_BlackBars_C|GetFadeIn _blackbars) 0.0 1 "Reverse" 1.0 false))))

(event Custom|StartCinematic
  (bind _blackbars (Variables|Default|GetBlackBars))
  ;[0.02922 0.15 0.0212 0.5] Leo's Black Bar
  (Utilities|IsValid _blackbars
    (:Is%20Valid
      (UserInterface|Animation|PlayAnimation _blackbars (Variables|/Game/07_UI/InGame/General/WBP_BlackBars.WBP_BlackBars_C|GetFadeIn _blackbars) 0.0 1 "Forward" 1.0 false))))

(event EventBeginPlay
  ;[0.02922 0.15 0.0212 0.5] Leo's Black Bar
  (Utilities|FlowControl|Sequence
    (:then_1
      (bind _returnvalue (UserInterface|CreateWidget "/Game/07_UI/InGame/General/WBP_BlackBars.WBP_BlackBars_C" (Game|GetPlayerController 0)))
      (UserInterface|Viewport|AddtoViewport _returnvalue 10)
      (Variables|Default|SetBlackBars _returnvalue))))

(event EventCloseSettingsinBlueprint
  ;[0.06787 0.4005 0.724 0.5] Close Settings Panel
  (Default|PushMenuWidget (Variables|Default|GetGameLayout) (Variables|Default|GetPreviousWidgetClass))
  (Default|RemoveWidget (Variables|Default|GetGameLayout) (Variables|Default|GetSettingsMenuWidgetInstance))
  (Variables|Default|SetSettingsMenuWidgetInstance 0))

(event EventOpenSettingsinBlueprint
  ;[0.06787 0.4005 0.724 0.5] Open Settings Panel
  (bind _widget (Default|PushMenuWidget (Variables|Default|GetGameLayout) (Variables|Default|GetSettingsMenuWidgetClass)))
  (bind _assettings_menu_widget (Utilities|Casting|CastToSettingsMenuWidget _widget))
  (Variables|Default|SetSettingsMenuWidgetInstance _assettings_menu_widget))

(event EventPauseGameinBlueprint
  ;[0.244 0.75 0.649 0.5] Open Pause Menu
  (bind _returnvalue (UserInterface|CreateWidget (Variables|Default|GetWBPGameLayout) (Game|GetPlayerController 0)))
  (bind _aswbp_game_layout (Utilities|Casting|CastToWBP_GameLayout _returnvalue))
  (bind _output_get (Variables|Default|SetGameLayout _aswbp_game_layout))
  (UserInterface|Viewport|AddtoViewport _output_get 1000000)
  (bind _widget (Default|PushMenuWidget (Variables|Default|GetGameLayout) (Variables|Default|GetPreviousWidgetClass)))
  (bind _asbase_menu_widget (Utilities|Casting|CastToBaseMenuWidget _widget))
  (Variables|Default|SetPreviousWidgetInstance _asbase_menu_widget))

(event EventResumeGameinBlueprint
  ;[0.244 0.75 0.649 0.5] Close Pause Menu
  (Widget|RemovefromParent (Variables|Default|GetGameLayout)))

(fn ConstructionScript)

(fn GetBlackBarPlayLength
  (bind _returnvalue (Animation|GetPlayLength (Variables|/Game/07_UI/InGame/General/WBP_BlackBars.WBP_BlackBars_C|GetFadeIn (Variables|Default|GetBlackBars))))
  (return _returnvalue))