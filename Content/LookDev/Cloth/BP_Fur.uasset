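; BP_Fur is a look-dev actor that builds shell-style fur by stacking copies of a mesh.
; Its construction script assigns the chosen mesh and material to an instanced static mesh component, then adds LayerNum instances at the same transform.
; Each instance stores its index and the total layer count as custom data, presumably so the material can offset and shade each shell.
; The event graph has no active logic.
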(event EventBeginPlay)

(event Collision|EventActorBeginOverlap
  (params (OtherActor :type Actor%20Object%20Reference)))

(event EventTick
  (params (DeltaSeconds :type Float%20%28single-precision%29)))

(fn ConstructionScript
  (bind _layernum (Variables|Default|GetLayerNum))
  (bind _instancedstaticmesh (Variables|Default|GetInstancedStaticMesh))
  (bind _instancedstaticmesh_2 (Variables|Default|GetInstancedStaticMesh))
  (bind _instancedstaticmesh_3 (Variables|Default|GetInstancedStaticMesh))
  (Components|StaticMesh|SetStaticMesh _instancedstaticmesh_3 (Variables|Default|GetStatic%20Mesh))
  (Rendering|Material|SetMaterial _instancedstaticmesh_3 0 (Variables|Default|GetMaterial))
  (Class|InstancedStaticMeshComponent|SetNumCustomDataFloats _instancedstaticmesh_3 2)
  (for _index (range 0 (- _layernum 1))
    (bind _returnvalue (Components|InstancedStaticMesh|AddInstance _instancedstaticmesh (Transformation|GetWorldTransform _instancedstaticmesh) true))
    (Components|InstancedStaticMesh|SetCustomDataValue _instancedstaticmesh_2 _returnvalue 0 (Math|Conversions|ToFloat(Integer) _returnvalue) false)
    (Components|InstancedStaticMesh|SetCustomDataValue _instancedstaticmesh_2 _returnvalue 1 (Math|Conversions|ToFloat(Integer) _layernum) false)
    (Components|InstancedStaticMesh|UpdateInstanceTransform _instancedstaticmesh_2 _returnvalue (Transformation|GetWorldTransform _instancedstaticmesh_2) true true false)))