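; Single-instance sky and weather actor that drives sun, skylight, height fog, volumetric clouds and weather FX from presets.
; ChangeSky loads a DT_Skys row and blends to it over a timeline through LerpSky; SetCustomSky applies settings immediately.
; UpdateSky pushes current settings to components, the cloud material, MPC_Sky and BP_SAS_Fx actors.
; Storm amounts above 0.5 randomly trigger BP_ThunderSpot effects; moon settings are blended but never applied.
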(event Custom|ChangeSky
  (params (SkyName :type String) (OverTime :type Float%20%28double-precision%29))
  (bind _returnvalue (Utilities|GetDataTableRow "/Game/super-adjustable-sky/Data/DT_Skys.DT_Skys" (Utilities|String|StringToName SkyName))
    (:then
      (Variables|Default|SetNewSettings _returnvalue)
      (Variables|Default|SetOld%20Settings (Variables|SkySettings|GetCurretSettings))
      (Components|Timeline|SetPlayRate (Variables|Default|GetTimeline) (/ 1.0 OverTime))
      (Variables|Default|SetbSwitchingSky true)
      (bind _timeline (Timeline|Timeline PlayFromStart)
        (:Update
          (CallFunction|LerpSky _timeline)
          (CallFunction|UpdateSky))
        (:Finished
          (Variables|Default|SetbSwitchingSky false))))))

(event Custom|SetCustomSky
  (params (Sky :type S%20Sky%20Preset%20Structure))
  (Variables|SkySettings|SetCurretSettings Sky)
  (CallFunction|UpdateSky)
  (CallFunction|UpdateWorldActorReferences))

(event Custom|UpdateWorldActorReferences
  (bind _outactors (Actor|GetAllActorsOfClass "/Game/super-adjustable-sky/BP/BP_ThunderSpot.BP_ThunderSpot_C"))
  (Variables|Default|SetThunderSpotsRefs _outactors)
  (bind _outactors_2 (Actor|GetAllActorsOfClass "/Game/super-adjustable-sky/BP/BP_SAS_Fx.BP_SAS_Fx_C"))
  (Variables|Default|SetFXSpotsRefs _outactors_2))

(event Collision|EventActorBeginOverlap
  (params (OtherActor :type Actor%20Object%20Reference)))

(event EventTick
  (params (DeltaSeconds :type Float%20%28single-precision%29))
  (bind _curretsettings (Variables|SkySettings|GetCurretSettings))
  (bind _thunderlikelyness (Variables|Default|GetThunderLikelyness))
  (bind _stormammount (Utilities|Struct|BreakS_SkyPreset _curretsettings))
  (bind _returnvalue (/ _thunderlikelyness _stormammount))
  (bind _returnvalue_2 (Math|Float|Truncate _returnvalue))
  (if (and (> _stormammount 0.5) (not (Variables|Default|GetbSwitchingSky)))
    (if (== (- _returnvalue_2 1) (Math|Random|RandomInteger _returnvalue_2))
      (Default|PlayFx (.OutItem (Utilities|Array|Random (Variables|Default|GetThunderSpotsRefs)))))))

(fn ConstructionScript
  (bind _sm_skysphere (Variables|Default|GetSM_SkySphere))
  ;[0.5469 0.474 0.0794 0.5] Just A Security
  (bind _outactors (Actor|GetAllActorsOfClass "BP_SuperAdjustableSky_C"))
  (if (> (Utilities|Array|Length _outactors) 1)
    (Development|PrintString "Warning ! More than one SAS in the scene || Super Adjustable Sky" true true "(R=1.000000,G=0.012506,B=0.000052,A=1.000000)" 99999999999999.0)
    (else
      (Transformation|SetActorLocation "0, 0, 0" false false)
      (Utilities|FlowControl|Sequence
        (:then_0
          ;[0.15 0.15 0.15 0.5] StoreAllTheSpotsForThunder
          (bind _outactors_2 (Actor|GetAllActorsOfClass "/Game/super-adjustable-sky/BP/BP_ThunderSpot.BP_ThunderSpot_C"))
          (Variables|Default|SetThunderSpotsRefs _outactors_2))
        (:then_1
          (bind _returnvalue (Utilities|GetDataTableRow "/Game/super-adjustable-sky/Data/DT_Skys.DT_Skys" "Morning_Cloudy")
            (:then
              (Variables|SkySettings|SetCurretSettings _returnvalue)
              (CallFunction|UpdateSky))))
        (:then_2
          (bind _returnvalue_2 (Rendering|Material|CreateDynamicMaterialInstance "/Game/super-adjustable-sky/_Core/Materials/m_SimpleVolumetricCloud_Inst.m_SimpleVolumetricCloud_Inst" "None" "None" :!class /Script/Engine.KismetMaterialLibrary))
          (Variables|Default|SetCloudMat _returnvalue_2)
          (Rendering|Material|SetMaterial (Variables|Default|GetVolumetricCloud) _returnvalue_2))
        (:then_3
          (bind _returnvalue_3 (Rendering|Material|CreateDynamicMaterialInstance (Rendering|Material|GetMaterial _sm_skysphere 0) "None" "None" :!class /Script/Engine.KismetMaterialLibrary))
          (bind _output_get (Variables|Default|SetSkydome%20Mat _returnvalue_3))
          (Rendering|Material|SetMaterial _sm_skysphere 0 _output_get))
        (:then_4
          (bind _outactors_3 (Actor|GetAllActorsOfClass "/Game/super-adjustable-sky/BP/BP_SAS_Fx.BP_SAS_Fx_C"))
          (Variables|Default|SetFXSpotsRefs _outactors_3))
        (:then_5
          (bind _foundwidgets (Widget|GetAllWidgetsOfClass "/Game/super-adjustable-sky/Tool/EUW_PresetSaver.EUW_PresetSaver_C" false))
          (for _array_element _foundwidgets
            _))))))

(fn UpdateSky
  (bind _curretsettings (Variables|SkySettings|GetCurretSettings))
  (bind _exponentialheightfog (Variables|Default|GetExponentialHeightFog))
  (bind _skylight (Variables|Default|GetSkyLight))
  (bind _cloudmat (Variables|Default|GetCloudMat))
  (bind _sun (Variables|Default|GetSun))
  (bind _thunderlikelyness (Variables|Default|GetThunderLikelyness))
  (bind (_stormammount _skycoverage _windintensity _windmap _precipitation _sunintensity _suncolor _sunsourceangle _sunsoftsourceangle _sunangle _moonintensity _mooncolor _moonsourceangle _moonsoftsourceangle _moonangle _skylightintensity _skylightcolor _foghight _fogdensity) (Utilities|Struct|BreakS_SkyPreset _curretsettings))
  (bind _returnvalue (/ _thunderlikelyness _stormammount))
  (bind _returnvalue_2 (Math|Float|Truncate _returnvalue))
  (Utilities|FlowControl|Sequence
    (:then_0
      (Transformation|SetWorldLocation _exponentialheightfog (Math|Vector|MakeVector 0.0 0.0 _foghight) false false)
      (Class|ExponentialHeightFogComponent|SetFogDensity _exponentialheightfog _fogdensity)
      (Rendering|Components|Light|SetIntensity _skylight _skylightintensity)
      (Rendering|Components|Light|SetLightColor _skylight (Math|Conversions|ToLinearColor(Color) _skylightcolor)))
    (:then_1
      (if (> _stormammount 0.5)
        (if (== (Math|Random|RandomInteger _returnvalue_2) (- _returnvalue_2 1))
          (Default|PlayFx (.OutItem (Utilities|Array|Random (Variables|Default|GetThunderSpotsRefs)))))))
    (:then_2
      (Rendering|Material|SetScalarParameterValue _cloudmat "Cloud_GlobalCoverage" _skycoverage :!class /Script/Engine.MaterialInstanceDynamic)
      (Rendering|Material|SetScalarParameterValue _cloudmat "UniformWindSpeed" _windintensity :!class /Script/Engine.MaterialInstanceDynamic)
      (Rendering|Material|SetScalarParameterValue _cloudmat "StormClouds" _stormammount :!class /Script/Engine.MaterialInstanceDynamic))
    (:then_3
      (Rendering|Components|Light|SetIntensity _sun _sunintensity)
      (Rendering|Components|Light|SetLightColor _sun (Math|Conversions|ToLinearColor(Color) _suncolor) true)
      (Class|DirectionalLightComponent|SetLightSourceAngle _sun _sunsourceangle)
      (Class|DirectionalLightComponent|SetLightSourceSoftAngle _sun _sunsoftsourceangle)
      (Transformation|SetWorldRotation _sun (Math|Conversions|RotationFromXVector _sunangle) false false))
    (:then_4
      (for _array_element (Variables|Default|GetFXSpotsRefs)
        (Default|Update _array_element _precipitation _windintensity)))
    (:then_5
      (Rendering|Material|SetScalarParameterValue "/Game/super-adjustable-sky/Data/MPC_Sky.MPC_Sky" "Precipitation" _precipitation :!class /Script/Engine.KismetMaterialLibrary)
      (Rendering|Material|SetScalarParameterValue "/Game/super-adjustable-sky/Data/MPC_Sky.MPC_Sky" "WindAmount" _windintensity :!class /Script/Engine.KismetMaterialLibrary))))

(fn LerpSky
  (params (Alpha :type Float%20%28double-precision%29))
  (bind _newsettings (Variables|Default|GetNewSettings))
  (bind _old_settings (Variables|Default|GetOld%20Settings))
  (bind (_stormammount _skycoverage _windintensity _windmap _precipitation _sunintensity _suncolor _sunsourceangle _sunsoftsourceangle _sunangle _moonintensity _mooncolor _moonsourceangle _moonsoftsourceangle _moonangle _skylightintensity _skylightcolor _foghight _fogdensity) (Utilities|Struct|BreakS_SkyPreset _newsettings))
  (bind (_stormammount_2 _skycoverage_2 _windintensity_2 _windmap_2 _precipitation_2 _sunintensity_2 _suncolor_2 _sunsourceangle_2 _sunsoftsourceangle_2 _sunangle_2 _moonintensity_2 _mooncolor_2 _moonsourceangle_2 _moonsoftsourceangle_2 _moonangle_2 _skylightintensity_2 _skylightcolor_2 _foghight_2 _fogdensity_2) (Utilities|Struct|BreakS_SkyPreset _old_settings))
  (Variables|SkySettings|SetCurretSettings (Utilities|Struct|MakeS_SkyPreset (Math|Float|Lerp _stormammount_2 _stormammount Alpha) (Math|Float|Lerp _skycoverage_2 _skycoverage Alpha) (Math|Float|Lerp _windintensity_2 _windintensity Alpha) 0 (Math|Float|Lerp _precipitation_2 _precipitation Alpha) (Math|Float|Lerp _sunintensity_2 _sunintensity Alpha) (Math|Conversions|ToColor(LinearColor) (Math|Color|Lerp(LinearColor) (Math|Conversions|ToLinearColor(Color) _suncolor_2) (Math|Conversions|ToLinearColor(Color) _suncolor) Alpha)) (Math|Float|Lerp _sunsourceangle_2 _sunsourceangle Alpha) (Math|Float|Lerp _sunsoftsourceangle_2 _sunsoftsourceangle Alpha) (Math|Vector|Lerp(Vector) _sunangle_2 _sunangle Alpha) (Math|Float|Lerp _moonintensity_2 _moonintensity Alpha) (Math|Conversions|ToColor(LinearColor) (Math|Color|Lerp(LinearColor) (Math|Conversions|ToLinearColor(Color) _mooncolor_2) (Math|Conversions|ToLinearColor(Color) _mooncolor) Alpha)) (Math|Float|Lerp _moonsourceangle_2 _moonsourceangle Alpha) (Math|Float|Lerp _moonsoftsourceangle_2 _moonsoftsourceangle Alpha) (Math|Vector|Lerp(Vector) _moonangle_2 _moonangle Alpha) (Math|Float|Lerp _skylightintensity_2 _skylightintensity Alpha) (Math|Conversions|ToColor(LinearColor) (Math|Color|Lerp(LinearColor) (Math|Conversions|ToLinearColor(Color) _skylightcolor_2) (Math|Conversions|ToLinearColor(Color) _skylightcolor) Alpha)) (Math|Float|Lerp _foghight_2 _foghight Alpha) (Math|Float|Lerp _fogdensity_2 _fogdensity Alpha))))