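; BP_ThunderSpot is a placeable lightning strike spot that plays a Niagara bolt effect on demand.
; The construction script moves the effect to BoltTop and converts BoltBottom from actor space into the component's local space to set the "Target Offset" parameter.
; It also disables the component's tick until the PlayFx event re-enables it and resets the system to fire the strike.
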(event Custom|Play%20Fx
  (bind _ns_lightning_strike (Variables|Default|GetNS_Lightning_Strike))
  (Components|Tick|SetComponentTickEnabled _ns_lightning_strike true)
  (Niagara|ResetSystem _ns_lightning_strike))

(event EventBeginPlay)

(event Collision|EventActorBeginOverlap
  (params (OtherActor :type Actor%20Object%20Reference)))

(event EventTick
  (params (DeltaSeconds :type Float%20%28single-precision%29)))

(fn ConstructionScript
  (bind _ns_lightning_strike (Variables|Default|GetNS_Lightning_Strike))
  (Components|Tick|SetComponentTickEnabled _ns_lightning_strike false)
  (Transformation|SetRelativeLocation _ns_lightning_strike (Variables|Default|GetBoltTop) false false)
  (Niagara|SetNiagaraVariable(Vector3) _ns_lightning_strike "Target Offset" (Math|Transform|InverseTransformLocation (Transformation|GetWorldTransform _ns_lightning_strike) (Math|Transform|TransformLocation (Transformation|GetActorTransform) (Variables|Default|GetBoltBottom)))))