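; BP_SAS_Fx is a weather-driven Niagara effect actor for the Super Adjustable Sky asset.
; The construction script assigns the configurable Niagara asset to its System component.
; Its Update event receives precipitation and wind amounts and forwards them to the system as float parameters.
; The same event toggles the system's active state, switching it off in near-zero wind when ShouldKillWhenNoWInd is set.
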(event Custom|Update
  (params (Precipitation :type Float%20%28double-precision%29) (WindAmmount :type Float%20%28double-precision%29))
  (bind _system (Variables|Default|GetSystem))
  (Utilities|FlowControl|Sequence
    (:then_0
      (if (and (Variables|Default|GetShouldKillWhenNoWInd) (< WindAmmount 0.1))
        (Variables|Default|SetbIsEneable false)
        (else
          (Variables|Default|SetbIsEneable true)))
      (Components|Activation|SetActive (Variables|Default|GetSystem) (Variables|Default|GetbIsEneable) false))
    (:then_2
      (Effects|Components|ParticleSystem|SetFloatParameter _system "Precipitation" Precipitation)
      (Effects|Components|ParticleSystem|SetFloatParameter _system "WindAmount" WindAmmount))))

(event EventBeginPlay)

(event Collision|EventActorBeginOverlap
  (params (OtherActor :type Actor%20Object%20Reference)))

(event EventTick
  (params (DeltaSeconds :type Float%20%28single-precision%29)))

(fn ConstructionScript
  (Class|NiagaraComponent|SetAsset (Variables|Default|GetSystem) (Variables|Default|GetNiagaraToUse) true))