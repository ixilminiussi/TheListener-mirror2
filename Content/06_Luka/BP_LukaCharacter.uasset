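; BP_LukaCharacter is Luka's character Blueprint, handling surface-based Wwise footsteps and subtitled speech.
; Each step alternates feet, offsetting a downward trace sideways from the capsule, perpendicular to velocity, to read the physical surface.
; Snow plays its sound and spawns a footprint actor turned to camera yaw, while wood only plays an indoor sound.
; Speak forwards Wwise events to the subtitled Ak component.
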(event EventBeginPlay
  (Pawn|Input|AddControllerPitchInput 0.0))

(event EventOnStep
  (params (Intensity :type Float%20%28single-precision%29))
  (bind (_transform _isvalidground) (CallFunction|ComputeFootstepInfo))
  (switch Utilities|FlowControl|Switch|SwitchonEPhysicalSurface _isvalidground
    (:SurfaceType1
      (Class|AkGameplayStatics|PostEvent "/Game/WwiseAudio/Events/Default_Work_Unit/foleys/play_footsteps_snow.play_footsteps_snow")
      (Game|SpawnActorfromClass "/Game/06_Luka/BP_Luka_Footstep.BP_Luka_Footstep_C" _transform "Undefined" "MultiplyWithRoot" 0 0))
    (:SurfaceType2
      (Class|AkGameplayStatics|PostEvent "/Game/WwiseAudio/Events/Default_Work_Unit/foleys/play_footsteps_inside.play_footsteps_inside"))))

(event Collision|EventActorBeginOverlap
  (params (OtherActor :type Actor%20Object%20Reference)))

(fn ConstructionScript)

(fn ComputeFootstepInfo
  (bind _charactermovement (Variables|Character|GetCharacterMovement))
  (bind _velocity (Variables|/Script/Engine.MovementComponent|GetVelocity _charactermovement))
  (Variables|Default|SetIsRightFootStep (not (Variables|Default|GetIsRightFootStep)))
  (bind _outhit (Collision|LineTraceByChannel (+ (Transformation|GetWorldLocation (Variables|Default|GetCapsuleComponent)) (* (Math|Vector|Normalize (Math|Vector|RotateVector (Math|Vector|MakeVector (.x _velocity) (.y _velocity) 0.0) "0.000000,-90.000000,0.000000")) (* (Variables|Default|GetLeftRightFootGap) (Math|Float|SelectFloat 1.0 -1.0 (Variables|Default|GetIsRightFootStep))))) (+ (+ (Transformation|GetWorldLocation (Variables|Default|GetCapsuleComponent)) (* (Math|Vector|Normalize (Math|Vector|RotateVector (Math|Vector|MakeVector (.x _velocity) (.y _velocity) 0.0) "0.000000,-90.000000,0.000000")) (* (Variables|Default|GetLeftRightFootGap) (Math|Float|SelectFloat 1.0 -1.0 (Variables|Default|GetIsRightFootStep))))) (* (Math|Vector|VectorDown) 1e+02)) "TraceTypeQuery1" false 0 "None"))
  (if (.bblockinghit _outhit)
    (return (Math|Transform|MakeTransform (.impactpoint _outhit) (Math|Rotator|MakeRotator 0.0 0.0 (.yaw (Transformation|GetWorldRotation (Variables|Default|GetCameraComponent))))) (Variables|/Script/PhysicsCore.PhysicalMaterial|GetSurfaceType (.physmat _outhit)))
    (else
      (return "" "SurfaceType_Default"))))

(fn Speak
  (params (Ak%20Event :type Ak%20Audio%20Event%20Object%20Reference))
  (Class|SubtitledAkComponent|PostSubtitledEvent (Variables|Default|GetBP_SubtitledAkComponent) Ak%20Event))