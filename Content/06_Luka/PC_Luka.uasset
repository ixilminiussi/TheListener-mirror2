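; Player controller for Luka that sets up PlayStation gamepad feedback and visuals when play begins.
; On BeginPlay it sets the DualSense LED color, turns mic and player LEDs off, and stops all trigger effects.
; If a connected DualSense, DualSense Edge or DualShock 4 is detected, it tells GI_Main to apply PlayStation visuals.
; Unconnected nodes keep examples of adaptive trigger effects for reference.
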(event Custom|CheckAndApplyPlaystationVisual
  (params (ControllerId :type Integer))
  ;[1 0.05459 0 0.5] Verifies if the connected gamepad is a PS gamepad and applies the visuals accordingly
  (bind _returnvalue (Class|SonyGamepadProxy|DeviceIsConnected ControllerId))
  (if _returnvalue
    (bind _returnvalue_2 (Class|SonyGamepadProxy|GetDeviceType))
    (if (Math|Boolean|ORBoolean (Utilities|Enum|Equal(Enum) _returnvalue_2 "DualSense") (Utilities|Enum|Equal(Enum) _returnvalue_2 "DualSenseEdge") (Utilities|Enum|Equal(Enum) _returnvalue_2 "DualShock4"))
      (bind _asgi_main (Utilities|Casting|CastToGI_Main (Game|GetGameInstance)))
      (Class|BaseGameInstance|ApplyPlaystationVisuals _asgi_main))))

(event EventBeginPlay
  (bind _returnvalue (Game|GetPlayerController 0))
  (bind _returnvalue_2 (Class|GameplayStatics|GetPlayerControllerID _returnvalue))
  ;[0.1993 0.8698 0.5684 0.5] Setup Controller Visuals
  (Utilities|IsValid _returnvalue
    (:Is%20Valid
      (CallFunction|CheckandApplyPlaystationVisual _returnvalue_2)
      (Class|SonyGamepadProxy|LedColorEffects _returnvalue_2 (Math|Color|MakeColor 150 150 170) 0.0 0.0)
      (Class|SonyGamepadProxy|LedMicEffects _returnvalue_2 "MicOff")
      (Class|DualSenseProxy|LedPlayerEffects _returnvalue_2 "Off" "Low")
      (Class|DualSenseProxy|StopAllTriggersEffects _returnvalue_2))))

(fn ConstructionScript)