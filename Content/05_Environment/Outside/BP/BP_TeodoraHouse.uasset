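; Blueprint for Teodora's house in the outside environment, providing a flickering light effect and a toggle for city lights.
; FlickerLight waits a random moment, then loops the LightFlicker timeline to drive light intensity from off to very bright, with a short random pause between replays.
; ActivateCityLights and DeactivateCityLights switch visibility without propagating to children.
; BeginPlay is empty, and none of these events are called within this Blueprint.
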(event Custom|FlickerLight
  (Utilities|FlowControl|Delay (Math|Random|RandomFloatinRange 0.0 1.0))
  (bind _alpha (Timeline|LightFlicker PlayFromStart)
    (:Update
      (Rendering|Components|Light|SetIntensity (Math|Float|Lerp 0.0 3e+05 _alpha)))
    (:Finished
      (Utilities|FlowControl|Delay (Math|Random|RandomFloatinRange 0.0 0.3))
      (Timeline|LightFlicker PlayFromStart))))

(event Custom|DeactivateCityLights
  (Rendering|SetVisibility false false))

(event Custom|ActivateCityLights
  (Rendering|SetVisibility true false))

(event EventBeginPlay)

(event Collision|EventActorBeginOverlap
  (params (OtherActor :type Actor%20Object%20Reference)))

(event EventTick
  (params (DeltaSeconds :type Float%20%28single-precision%29)))

(fn ConstructionScript)