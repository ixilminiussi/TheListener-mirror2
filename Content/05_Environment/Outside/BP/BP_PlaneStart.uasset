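; BP_PlaneStart is an outdoor environment actor that shows a plane flying along once activated.
; The plane is hidden at BeginPlay, and the Activate override calls its parent, sets IsFlying, reveals the plane and plays a 2D plane sound.
; While flying, Tick moves the plane along relative Y by Speed each frame with sweep, without delta-time scaling.
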(event EventBeginPlay
  (Rendering|SetVisibility (Variables|Default|GetPlane) false false))

(event EventTick
  (params (DeltaSeconds :type Float%20%28single-precision%29))
  (bind _plane (Variables|Default|GetPlane))
  (if (Variables|Default|GetIsFlying?)
    (Transformation|SetRelativeLocation _plane (Math|Vector|MakeVector 0.0 (+ (.y (Variables|/Script/Engine.SceneComponent|GetRelativeLocation _plane)) (Variables|Default|GetSpeed)) 0.0) true false)))

(fn ConstructionScript)

(fn Activate
  (|CallParentFunction)
  (Variables|Default|SetIsFlying? true)
  (Rendering|SetVisibility (Variables|Default|GetPlane) true false)
  (Audio|PlaySound2D "/Game/05_Environment/Outside/Sound_placeholder/plane-78723.plane-78723" 1.0 1.0 0.0 0 0))