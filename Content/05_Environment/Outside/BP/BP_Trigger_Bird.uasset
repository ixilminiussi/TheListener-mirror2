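; BP_Trigger_Bird is a one-shot trigger volume that starts environment effects, presumably birds given its name, when something overlaps its box.
; The first overlap, with no check on the overlapping actor, passes a DoOnce and activates the Niagara component of each actor in NiagaraToActivate.
; It then calls Activate on each entry in EnviroElementsToActivate.
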(event OnComponentBeginOverlap(Box)
  (params (OverlappedComponent :type Primitive%20Component%20Object%20Reference) (OtherActor :type Actor%20Object%20Reference) (OtherComp :type Primitive%20Component%20Object%20Reference) (OtherBodyIndex :type Integer) (bFromSweep :type Boolean) (SweepResult :type Hit%20Result%20Structure%20%28by%20ref%29))
  (bind _enviroelementstoactivate (Variables|Default|GetEnviroElementsToActivate))
  (bind _niagaratoactivate (Variables|Default|GetNiagaraToActivate))
  (Utilities|FlowControl|DoOnce false
    (:Completed
      (Utilities|FlowControl|Sequence
        (:then_0
          (if (not (Utilities|Array|IsEmpty _niagaratoactivate))
            (for _array_element _niagaratoactivate
              (Components|Activation|Activate (Variables|/Script/Niagara.NiagaraActor|GetNiagaraComponent _array_element) false))))
        (:then_1
          (if (not (Utilities|Array|IsEmpty _enviroelementstoactivate))
            (for _array_element_2 _enviroelementstoactivate
              (Default|Activate _array_element_2))))))))

(event EventBeginPlay)

(event Collision|EventActorBeginOverlap
  (params (OtherActor :type Actor%20Object%20Reference)))

(event EventTick
  (params (DeltaSeconds :type Float%20%28single-precision%29)))

(fn ConstructionScript)