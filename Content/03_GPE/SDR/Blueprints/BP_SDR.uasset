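; BP_SDR is the Blueprint for a radio device (SDR) with switchable LF, MF and HF bands.
; SetBand swaps the screen's renderer material, the band label text and the switch's colored light material to match the selected band.
; AddBand reveals a wire mesh, hidden at BeginPlay, and calls AllowBand to unlock the band, handling only the first two bands.
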(event EventBeginPlay
  (Rendering|SetVisibility (Variables|Default|GetWireRef) false false))

(event EventSetBand
  (params (Band :type Integer))
  (switch int Band
    (:0
      (Rendering|Material|SetMaterial (Variables|Default|GetSM_Screen) 0 "/Game/03_GPE/SDR/Materials/MI_LFRenderer.MI_LFRenderer")
      (Rendering|Components|TextRender|SetText (Variables|Default|GetBandExternalText) (Variables|Default|GetLFText))
      (Rendering|Material|SetMaterial (Variables|Default|GetSM_SDR_FMSwitch) 4 "/Game/03_GPE/Radio/Materials/Decoder/MI_GreenLight.MI_GreenLight"))
    (:1
      (Rendering|Material|SetMaterial (Variables|Default|GetSM_Screen) 0 "/Game/03_GPE/SDR/Materials/MI_MFRenderer.MI_MFRenderer")
      (Rendering|Components|TextRender|SetText (Variables|Default|GetBandExternalText) (Variables|Default|GetMFText))
      (Rendering|Material|SetMaterial (Variables|Default|GetSM_SDR_FMSwitch) 4 "/Game/03_GPE/Radio/Materials/Decoder/MI_BlueLight.MI_BlueLight"))
    (:2
      (Rendering|Material|SetMaterial (Variables|Default|GetSM_Screen) 0 "/Game/03_GPE/SDR/Materials/MI_HFRenderer.MI_HFRenderer")
      (Rendering|Components|TextRender|SetText (Variables|Default|GetBandExternalText) (Variables|Default|GetHFText))
      (Rendering|Material|SetMaterial (Variables|Default|GetSM_SDR_FMSwitch) 4 "/Game/03_GPE/Radio/Materials/Decoder/MI_RedLight.MI_RedLight"))))

(fn ConstructionScript)

(fn AddBand
  (params (NewParam :type Integer))
  (switch int NewParam
    (:0
      (Rendering|SetVisibility (Variables|Default|GetWireRef) true false))
    (:1
      (Rendering|SetVisibility (Variables|Default|GetWireRef) true false)))
  (Class|TLUtils|AllowBand self NewParam))