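; BP_CloseDoor is a trigger box that closes a door when entered.
; It overrides EnterBox and, after the parent logic, checks CanCloseDoor before calling CloseDoor on the BP_Door found via GetActorOfClass.
; It then calls the enter-box event and destroys itself, so it closes the door only once.
; The lookup is by class, so it targets whichever single BP_Door is returned rather than an assigned reference.
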(event EventBeginPlay
  (|CallParentFunction) ; This node is disabled and will not be called.\nDrag off pins to build functionality.
)

(event Collision|EventActorBeginOverlap
  (params (OtherActor :type Actor%20Object%20Reference))
  (|CallParentFunction OtherActor) ; This node is disabled and will not be called.\nDrag off pins to build functionality.
)

(event EventTick
  (params (DeltaSeconds :type Float%20%28single-precision%29))
  (|CallParentFunction DeltaSeconds) ; This node is disabled and will not be called.\nDrag off pins to build functionality.
)

(fn ConstructionScript
  (|CallParentFunction))

(fn EnterBox
  (|CallParentFunction)
  (if (Variables|Default|GetCanCloseDoor)
    (bind _returnvalue (Actor|GetActorOfClass "/Game/03_GPE/Interactables/BP_Door.BP_Door_C"))
    (Default|CloseDoor _returnvalue)
    (Default|CallEnterBoxEvent)
    (Actor|DestroyActor)))