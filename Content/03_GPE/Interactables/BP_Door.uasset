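; BP_Door is an interactable door that swings open by rotating the whole actor around yaw.
; BeginPlay caches the closed rotation and derives the open one by adding ValueToTurn to its yaw.
; OnInteract plays a Wwise sound, calls Enable(false) and lerps to the open rotation on a timeline.
; CloseDoor lerps back on a second timeline with its own sound, without calling Enable again.
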(event Custom|CloseDoor
  (Class|AkGameplayStatics|PostEvent "/Game/WwiseAudio/Events/Default_Work_Unit/foleys/play_close_door.play_close_door")
  (bind _alpha (Timeline|Timeline PlayFromStart)
    (:Update
      (Transformation|SetActorRotation (Math|Rotator|Lerp(Rotator) (Variables|Default|GetTargetRota) (Variables|Default|GetBasicRota) _alpha)))))

(event EventBeginPlay
  (bind _output_get (Variables|Default|SetBasicRota (Transformation|GetActorRotation)))
  (Variables|Default|SetTargetRota (Math|Rotator|MakeRotator (.roll _output_get) (.pitch _output_get) (+ (.yaw _output_get) (Variables|Default|GetValueToTurn)))))

(event Collision|EventActorBeginOverlap
  (params (OtherActor :type Actor%20Object%20Reference)))

(event EventTick
  (params (DeltaSeconds :type Float%20%28single-precision%29)))

(event EventOnInteract
  (Class|AkGameplayStatics|PostEvent "/Game/WwiseAudio/Events/Default_Work_Unit/foleys/play_open_door.play_open_door")
  (Class|Interactable|Enable false)
  (bind _alpha (Timeline|DoorOpen PlayFromStart)
    (:Update
      (Transformation|SetActorRotation (Math|Rotator|Lerp(Rotator) (Variables|Default|GetBasicRota) (Variables|Default|GetTargetRota) _alpha)))))

(fn ConstructionScript)