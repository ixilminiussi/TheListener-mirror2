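; BP_LowFrequencyWire is a low-frequency wire object that can be dropped at a designated location.
; It starts disabled, then after a delay registers a drop location at the BP_LowFrequencyWireReference actor's root transform and deactivates that actor.
; When dropped, it activates the reference actor, destroys itself and signals that the wire is dropped, so the placed reference stands in for it.
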(event EventBeginPlay
  (Class|Interactable|Enable false)
  (Utilities|FlowControl|Delay 8.0)
  (bind _returnvalue (Actor|GetActorOfClass "/Game/03_GPE/Objis/Blueprints/BP_LowFrequencyWireReference.BP_LowFrequencyWireReference_C"))
  (Utilities|IsValid _returnvalue
    (:Is%20Valid
      (CallFunction|AddDropLocation (Transformation|GetWorldTransform (Variables|/Script/Engine.Actor|GetRootComponent _returnvalue)) 5e+01)
      (Default|Deactivate _returnvalue))))

(event Collision|EventActorBeginOverlap
  (params (OtherActor :type Actor%20Object%20Reference)))

(event EventTick
  (params (DeltaSeconds :type Float%20%28single-precision%29)))

(event EventOnDrop
  (bind _returnvalue (Actor|GetActorOfClass "/Game/03_GPE/Objis/Blueprints/BP_LowFrequencyWireReference.BP_LowFrequencyWireReference_C"))
  (Default|Activate _returnvalue)
  (Actor|DestroyActor)
  (Default|CallLowFrequencyWireIsDropped))

(fn ConstructionScript)