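; BP_WoodPile is a wood pile object with a drop point, which slows Luka while it exists, apparently as a carried load.
; After a short BeginPlay delay, it registers the BP_WoodPileReference actor's transform as a drop location, deactivates that actor and lowers Luka's walk speed.
; On drop, it reactivates the reference actor, raises the walk speed again and destroys itself.
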(event EventBeginPlay
  (Utilities|FlowControl|Delay 0.2)
  (bind _returnvalue (Actor|GetActorOfClass "/Game/03_GPE/Objis/Blueprints/BP_WoodPileReference.BP_WoodPileReference_C"))
  (Utilities|IsValid _returnvalue
    (:Is%20Valid
      (Class|FixedPlacementObji|AddDropLocation (Transformation|GetWorldTransform (Variables|/Script/Engine.Actor|GetRootComponent _returnvalue)) 5e+01)
      (Default|Deactivate _returnvalue)
      (Utilities|FlowControl|Delay 0.05)
      (bind _asluka_character (Utilities|Casting|CastToLukaCharacter (Game|GetPlayerCharacter 0)))
      (Variables|/Script/Engine.CharacterMovementComponent|SetMaxWalkSpeed (Variables|/Script/Engine.Character|GetCharacterMovement _asluka_character) 1.7e+02))))

(event Collision|EventActorBeginOverlap
  (params (OtherActor :type Actor%20Object%20Reference)))

(event EventTick
  (params (DeltaSeconds :type Float%20%28single-precision%29)))

(event EventOnDrop
  (bind _returnvalue (Actor|GetActorOfClass "/Game/03_GPE/Objis/Blueprints/BP_WoodPileReference.BP_WoodPileReference_C"))
  (Default|Activate _returnvalue)
  (bind _asluka_character (Utilities|Casting|CastToLukaCharacter (Game|GetPlayerCharacter 0)))
  (Variables|/Script/Engine.CharacterMovementComponent|SetMaxWalkSpeed (Variables|/Script/Engine.Character|GetCharacterMovement _asluka_character) 2.5e+02)
  (Actor|DestroyActor))

(fn ConstructionScript)