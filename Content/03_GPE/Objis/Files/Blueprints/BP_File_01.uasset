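; BP_File_01 is a file object that plays Wwise audio when it is picked up or dropped.
; OnPickup and OnDrop post OnPickEvent and OnDropEvent respectively on its AkComponent, after checking that both the event and the component are valid.
; The graphs hold no other logic, and the construction script is empty.
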(event EventOnDrop
  (Utilities|IsValid (Variables|Default|GetOnDropEvent)
    (:Is%20Valid
      (Utilities|IsValid (Variables|Default|GetAkComponent)
        (:Is%20Valid
          (Class|AkGameObject|PostAkEvent (Variables|Default|GetAkComponent) (Variables|Default|GetOnDropEvent)))))))

(event EventOnPickup
  (Utilities|IsValid (Variables|Default|GetOnPickEvent)
    (:Is%20Valid
      (Utilities|IsValid (Variables|Default|GetAkComponent)
        (:Is%20Valid
          (Class|AkGameObject|PostAkEvent (Variables|Default|GetAkComponent) (Variables|Default|GetOnPickEvent)))))))

(fn ConstructionScript)