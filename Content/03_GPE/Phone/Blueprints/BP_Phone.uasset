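; BP_Phone is a possessable phone that shows an input number on digit actors and displays a phone directory widget.
; On BeginPlay it creates the directory widget and adds it to the viewport, then opens it after a possession transition and closes it before unpossession.
; On each number update it clears every BP_NumberDigit child actor, then sets each input digit on the display at the matching index.
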(event EventOnNumberUpdate
  (params (NumberInput :type Array%20of%20Integers))
  (for _array_element (Variables|Default|GetNumberDigits)
    (bind _asbp_number_digit (Utilities|Casting|CastToBP_NumberDigit (Variables|/Script/Engine.ChildActorComponent|GetChildActor _array_element)))
    (Default|Clear _asbp_number_digit))
  (for (_array_element_2 _array_index) NumberInput
    (bind _asbp_number_digit_2 (Utilities|Casting|CastToBP_NumberDigit (Variables|/Script/Engine.ChildActorComponent|GetChildActor (Utilities|Array|Get(acopy) (Variables|Default|GetNumberDigits) _array_index))))
    (Default|SetNumber _asbp_number_digit_2 _array_element_2)))

(event EventOnUnPossessBeforeTransition
  (Default|CloseDirectory (Variables|Default|GetPhoneDirectory)))

(event EventOnPossessAfterTransition
  (Default|OpenDirectory (Variables|Default|GetPhoneDirectory)))

(event EventBeginPlay
  (bind _returnvalue (UserInterface|CreateWidget "/Game/07_UI/Phone/W_PhoneDirectoryTest.W_PhoneDirectoryTest_C"))
  (bind _output_get (Variables|Default|SetPhoneDirectory _returnvalue))
  (UserInterface|Viewport|AddtoViewport _output_get 0))

(fn ConstructionScript)