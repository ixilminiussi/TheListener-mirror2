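; Seven-segment display actor for the phone that shows a single digit from 0 to 9 using static mesh segments SM1 to SM7.
; SetNumber first calls Clear, which resets every segment to the grey material, then switches on the number and sets the matching segments to the green light material.
; The event graph is unused, so the display only changes when SetNumber or Clear is called.
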(event EventBeginPlay)

(event Collision|EventActorBeginOverlap
  (params (OtherActor :type Actor%20Object%20Reference)))

(event EventTick
  (params (DeltaSeconds :type Float%20%28single-precision%29)))

(fn ConstructionScript)

(fn SetNumber
  (params (Number :type Integer))
  (CallFunction|Clear)
  (switch int Number
    (:0
      (Utilities|FlowControl|Sequence
        (:then_0
          ;[0.08283 1 0 0.5] turn on
          (Rendering|Material|SetMaterial (Variables|Default|GetSM_1) 0 "/Game/03_GPE/Radio/Materials/Decoder/M_GreenLight.M_GreenLight" :!label _label))
        (:then_1
          (Rendering|Material|SetMaterial (Variables|Default|GetSM_2) 0 "/Game/03_GPE/Radio/Materials/Decoder/M_GreenLight.M_GreenLight" :!label _label_2))
        (:then_2
          (Rendering|Material|SetMaterial (Variables|Default|GetSM_3) 0 "/Game/03_GPE/Radio/Materials/Decoder/M_GreenLight.M_GreenLight" :!label _label_3))
        (:then_3
          (Rendering|Material|SetMaterial (Variables|Default|GetSM_5) 0 "/Game/03_GPE/Radio/Materials/Decoder/M_GreenLight.M_GreenLight" :!label _label_4))
        (:then_4
          (Rendering|Material|SetMaterial (Variables|Default|GetSM_6) 0 "/Game/03_GPE/Radio/Materials/Decoder/M_GreenLight.M_GreenLight" :!label _label_5))
        (:then_5
          (Rendering|Material|SetMaterial (Variables|Default|GetSM_7) 0 "/Game/03_GPE/Radio/Materials/Decoder/M_GreenLight.M_GreenLight" :!label _label_6))))
    (:1
      (Utilities|FlowControl|Sequence
        (:then_0
          (goto _label_3))
        (:then_1
          (goto _label_6))))
    (:2
      (Utilities|FlowControl|Sequence
        (:then_0
          (goto _label_2))
        (:then_1
          (goto _label_3))
        (:then_2
          (Rendering|Material|SetMaterial (Variables|Default|GetSM_4) 0 "/Game/03_GPE/Radio/Materials/Decoder/M_GreenLight.M_GreenLight" :!label _label_7))
        (:then_3
          (goto _label_4))
        (:then_4
          (goto _label_5))))
    (:3
      (Utilities|FlowControl|Sequence
        (:then_0
          (goto _label_2))
        (:then_1
          (goto _label_3))
        (:then_2
          (goto _label_7))
        (:then_3
          (goto _label_5))
        (:then_4
          (goto _label_6))))
    (:4
      (Utilities|FlowControl|Sequence
        (:then_0
          (goto _label))
        (:then_1
          (goto _label_3))
        (:then_2
          (goto _label_7))
        (:then_3
          (goto _label_6))))
    (:5
      (Utilities|FlowControl|Sequence
        (:then_0
          (goto _label))
        (:then_1
          (goto _label_2))
        (:then_2
          (goto _label_7))
        (:then_3
          (goto _label_5))
        (:then_4
          (goto _label_6))))
    (:6
      (Utilities|FlowControl|Sequence
        (:then_0
          (goto _label))
        (:then_1
          (goto _label_2))
        (:then_2
          (goto _label_7))
        (:then_3
          (goto _label_4))
        (:then_4
          (goto _label_5))
        (:then_5
          (goto _label_6))))
    (:7
      (Utilities|FlowControl|Sequence
        (:then_0
          (goto _label_2))
        (:then_1
          (goto _label_3))
        (:then_2
          (goto _label_6))))
    (:8
      (Utilities|FlowControl|Sequence
        (:then_0
          (goto _label))
        (:then_1
          (goto _label_2))
        (:then_2
          (goto _label_3))
        (:then_3
          (goto _label_7))
        (:then_4
          (goto _label_4))
        (:then_5
          (goto _label_5))
        (:then_6
          (goto _label_6))))
    (:9
      (Utilities|FlowControl|Sequence
        (:then_0
          (goto _label))
        (:then_1
          (goto _label_2))
        (:then_2
          (goto _label_3))
        (:then_3
          (goto _label_7))
        (:then_4
          (goto _label_5))
        (:then_5
          (goto _label_6))))))

(fn Clear
  ;[1 0.04365 0 0.5] turn off
  (Rendering|Material|SetMaterial (Variables|Default|GetSM_1) 0 "/Engine/EditorMeshes/ColorCalibrator/M_GreyBall.M_GreyBall")
  (Rendering|Material|SetMaterial (Variables|Default|GetSM_2) 0 "/Engine/EditorMeshes/ColorCalibrator/M_GreyBall.M_GreyBall")
  (Rendering|Material|SetMaterial (Variables|Default|GetSM_3) 0 "/Engine/EditorMeshes/ColorCalibrator/M_GreyBall.M_GreyBall")
  (Rendering|Material|SetMaterial (Variables|Default|GetSM_4) 0 "/Engine/EditorMeshes/ColorCalibrator/M_GreyBall.M_GreyBall")
  (Rendering|Material|SetMaterial (Variables|Default|GetSM_5) 0 "/Engine/EditorMeshes/ColorCalibrator/M_GreyBall.M_GreyBall")
  (Rendering|Material|SetMaterial (Variables|Default|GetSM_6) 0 "/Engine/EditorMeshes/ColorCalibrator/M_GreyBall.M_GreyBall")
  (Rendering|Material|SetMaterial (Variables|Default|GetSM_7) 0 "/Engine/EditorMeshes/ColorCalibrator/M_GreyBall.M_GreyBall"))