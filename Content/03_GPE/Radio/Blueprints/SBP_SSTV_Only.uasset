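; Radio station Blueprint for an SSTV-only broadcast, which yields a printed item once decoded.
; Entering and leaving station range starts and stops the decoder.
; On decode, it clears the decoder-active flag and finds the SSTV printer actor in the level.
; If the printer exists, it spawns the station asset's SSTV class at the printer's spawn point, calls NewSDRDoc on it and stops the station.
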(event EventBeginPlay)

(event Collision|EventActorBeginOverlap
  (params (OtherActor :type Actor%20Object%20Reference)))

(event EventTick
  (params (DeltaSeconds :type Float%20%28single-precision%29)))

(event EventOnDecoded
  (Variables|Default|SetDecoderActive false)
  (bind _returnvalue (Actor|GetActorOfClass "/Game/03_GPE/SSTV/BP_SSTV_Printer.BP_SSTV_Printer_C"))
  (Utilities|IsValid _returnvalue
    (:Is%20Valid
      (Game|SpawnActorfromClass (Variables|/Script/TheListener.StationAsset|GetSSTVClass (Variables|Default|GetStationAsset)) (Math|Transform|MakeTransform (.location (Transformation|GetWorldTransform (Variables|/Game/03_GPE/SSTV/BP_SSTV_Printer.BP_SSTV_Printer_C|GetSpawnPosition _returnvalue))) (.rotation (Transformation|GetWorldTransform (Variables|/Game/03_GPE/SSTV/BP_SSTV_Printer.BP_SSTV_Printer_C|GetSpawnPosition _returnvalue)))) "Undefined" "MultiplyWithRoot" 0 0)
      (Default|NewSDRDoc _returnvalue)
      (Class|Station|StopStation))))

(event EventOnEnteringStationRange
  (Class|Station|StartDecoder))

(event EventOnLeavingStationRange
  (Class|Station|StopDecoder))

(fn ConstructionScript)