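; SBP_Decoder is a radio station Blueprint for a coded number station that has to be decoded.
; On initialization it posts the coded-station Wwise event and prevents the end dialogue.
; Entering or leaving station range starts or stops the decoder until it is decoded.
; Decoding sets a flag, starts the station, stops the coded audio and calls Lock.
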(event EventBeginPlay)

(event Collision|EventActorBeginOverlap
  (params (OtherActor :type Actor%20Object%20Reference)))

(event EventTick
  (params (DeltaSeconds :type Float%20%28single-precision%29)))

(event EventInitialize
  (Class|AkGameObject|PostAkEvent (Variables|Default|GetAkComponent) "/Game/WwiseAudio/Events/DAY_2/Stations/play_number_station_coded.play_number_station_coded")
  (Class|Station|PreventEndDialogue))

(event EventOnEnteringStationRange
  (if (not (Variables|Default|GetIsDecoded))
    (Class|Station|StartDecoder)))

(event EventOnDecoded
  (Variables|Default|SetIsDecoded true)
  (Class|Station|StartStation)
  (Class|AkGameObject|PostAkEvent (Variables|Default|GetAkComponent) "/Game/WwiseAudio/Events/DAY_2/Stations/stop_number_station_coded.stop_number_station_coded")
  (Class|Dialogue|Lock true))

(event EventOnLeavingStationRange
  (if (not (Variables|Default|GetIsDecoded))
    (Class|Station|StopDecoder)))

(fn ConstructionScript)