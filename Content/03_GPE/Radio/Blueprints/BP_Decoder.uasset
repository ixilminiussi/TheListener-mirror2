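; BP_Decoder is a radio decoder device with two knobs, two status LEDs and a screen, handling its audio, haptic and visual feedback.
; On BeginPlay it binds both knobs' click events and adds a force feedback component; each click posts that knob's Wwise sound and spawns rumble.
; Toggle events swap BodyMesh material slots to show each LED as off, right (green) or wrong (red), and the screen as running or off.
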(event Custom|OnRightClick_Event
  (params (IsIncreasing :type Boolean))
  (bind _rightknobcomponent (Variables|Default|GetRightKnobComponent))
  (bind _startclickaudioevent (Variables|/Script/TheListener.KnobComponent|GetStartClickAudioEvent _rightknobcomponent))
  (bind _clickakcomponent (Variables|/Script/TheListener.KnobComponent|GetClickAkComponent _rightknobcomponent))
  ;[1 0.6632 0 0.5] Click Feedback
  (Utilities|IsValid _rightknobcomponent
    (:Is%20Valid
      (Utilities|IsValid _clickakcomponent
        (:Is%20Valid
          (Utilities|IsValid _startclickaudioevent
            (:Is%20Valid
              (Class|AkGameObject|PostAkEvent _clickakcomponent _startclickaudioevent)
              (ForceFeedback|SpawnForceFeedbackAttached "/Game/03_GPE/Radio/Blueprints/Feedbacks/FFE_ClickRadio.FFE_ClickRadio" (Variables|Default|GetRumbleKnob) "None" "0, 0, 0" "0, 0, 0" "KeepRelativeOffset" false false 1.0 0.0 0))))))))

(event Custom|OnLeftClick_Event
  (params (IsIncreasing :type Boolean))
  (bind _leftknobcomponent (Variables|Default|GetLeftKnobComponent))
  (bind _startclickaudioevent (Variables|/Script/TheListener.KnobComponent|GetStartClickAudioEvent _leftknobcomponent))
  (bind _clickakcomponent (Variables|/Script/TheListener.KnobComponent|GetClickAkComponent _leftknobcomponent))
  ;[1 0.6632 0 0.5] Click Feedback
  (Utilities|IsValid _leftknobcomponent
    (:Is%20Valid
      (Utilities|IsValid _clickakcomponent
        (:Is%20Valid
          (Utilities|IsValid _startclickaudioevent
            (:Is%20Valid
              (Class|AkGameObject|PostAkEvent _clickakcomponent _startclickaudioevent)
              (ForceFeedback|SpawnForceFeedbackAttached "/Game/03_GPE/Radio/Blueprints/Feedbacks/FFE_ClickRadio.FFE_ClickRadio" (Variables|Default|GetRumbleKnob) "None" "0, 0, 0" "0, 0, 0" "KeepRelativeOffset" false false 1.0 0.0 0))))))))

(event EventOnScreenToggle
  (params (bToggle :type Boolean))
  ;[0.15 0.15 0.15 0.5] ScreenToggle
  (Rendering|Material|SetMaterial (Variables|Default|GetBodyMesh) 3 (select bToggle (Variables|Default|GetRunningMaterialInstance) "/Game/UltraDynamicSky/Materials/Material_Instances/Lens_Flares/35mm_Prime.35mm_Prime")))

(event EventOnRightToggle
  (params (bToggle :type ELedState%20Enum :default "Off"))
  ;[1 0.03646 0.04945 0.5] Right LED
  (Rendering|Material|SetMaterial (Variables|Default|GetBodyMesh) 2 (Utilities|Select :Index bToggle :Off "/Game/UltraDynamicSky/Materials/Material_Instances/Lens_Flares/35mm_Prime.35mm_Prime" :Right "/Game/03_GPE/Radio/Materials/Decoder/M_GreenLight.M_GreenLight" :Wrong "/Game/03_GPE/Radio/Materials/Decoder/M_RedLight.M_RedLight")))

(event EventOnLeftToggle
  (params (bToggle :type ELedState%20Enum :default "Off"))
  ;[1 0 0.04659 0.5] Left LED
  (Rendering|Material|SetMaterial (Variables|Default|GetBodyMesh) 1 (Utilities|Select :Index bToggle :Off "/Game/UltraDynamicSky/Materials/Material_Instances/Lens_Flares/35mm_Prime.35mm_Prime" :Right "/Game/03_GPE/Radio/Materials/Decoder/M_GreenLight.M_GreenLight" :Wrong "/Game/03_GPE/Radio/Materials/Decoder/M_RedLight.M_RedLight")))

(event EventBeginPlay
  (bind _leftknobcomponent (Variables|Default|GetLeftKnobComponent))
  (bind _rightknobcomponent (Variables|Default|GetRightKnobComponent))
  (Utilities|IsValid _leftknobcomponent
    (:Is%20Valid
      (EventDispatchers|BindEventtoOnClick _leftknobcomponent (delegate Custom|OnLeftClick_Event))
      (Utilities|IsValid _rightknobcomponent
        (:Is%20Valid
          (EventDispatchers|BindEventtoOnClick _rightknobcomponent (delegate Custom|OnRightClick_Event))
          (bind _returnvalue (AddComponent|AddForceFeedbackComponent false (Transformation|GetActorTransform)))
          (Variables|Default|SetRumbleKnob _returnvalue))))))

(fn ConstructionScript)