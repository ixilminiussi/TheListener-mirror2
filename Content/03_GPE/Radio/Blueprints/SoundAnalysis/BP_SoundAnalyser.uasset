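; Audio spectrum visualizer actor that plays a Wwise debug music event and shows its frequency content as a row of cubes.
; On BeginPlay it posts the event and spawns 48 BP_Cube actors spaced along world Y.
; Each tick it uses the Wwise play position to sample precomputed, non-real-time Constant-Q data for channel 0.
; Each normalized band value drives the Z scale of its matching cube.
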(event EventBeginPlay
  (bind _returnvalue (Class|AkGameplayStatics|PostEvent "/Game/WwiseAudio/Events/Default_Work_Unit/debug/play_debug_music.play_debug_music" self 3145728))
  (Variables|Default|SetPlayingId _returnvalue)
  (CallFunction|SpawnSoundCubes 48 55.0))

(event EventTick
  (params (DeltaSeconds :type Float%20%28single-precision%29))
  (bind _returnvalue (Class|TLUtils|GetPlayPosition (Variables|Default|GetPlayingId)))
  (for (_array_element _array_index) (Class|ConstantQNRT|GetNormalizedChannelConstantQatTime (Variables|Default|GetConstantQNRT) (/ (Math|Conversions|ToFloat(Integer) _returnvalue) 1e+03))
    (Transformation|SetWorldScale3D (Variables|/Script/Engine.Actor|GetRootComponent (Utilities|Array|Get(acopy) (Variables|Default|GetCubes) _array_index)) (Math|Vector|MakeVector (.x (Transformation|GetWorldScale (Variables|/Script/Engine.Actor|GetRootComponent (Utilities|Array|Get(acopy) (Variables|Default|GetCubes) _array_index)))) (.y (Transformation|GetWorldScale (Variables|/Script/Engine.Actor|GetRootComponent (Utilities|Array|Get(acopy) (Variables|Default|GetCubes) _array_index)))) (* _array_element 15.0)))))

(fn ConstructionScript)

(fn SpawnSoundCubes
  (params (NumCubes :type Integer) (CubeSpace :type Float%20%28double-precision%29))
  (bind _defaultsceneroot (Variables|Default|GetDefaultSceneRoot))
  (bind _returnvalue (Transformation|GetWorldLocation _defaultsceneroot))
  (for _index (range 1 NumCubes)
    (bind _returnvalue_2 (Game|SpawnActorfromClass "/Game/03_GPE/Radio/Blueprints/SoundAnalysis/BP_Cube.BP_Cube_C" (Math|Transform|MakeTransform (Math|Vector|MakeVector (.x _returnvalue) (Math|Conversions|ToFloat(Integer) (* _index CubeSpace)) (.z _returnvalue)) "0, 0, 0" "1.000000,1.000000,1.000000") "Undefined" "MultiplyWithRoot" 0 0))
    (Utilities|Array|Add (Variables|Default|GetCubes) _returnvalue_2))
  (return (Variables|Default|GetCubes)))