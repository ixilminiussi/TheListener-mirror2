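; Radio station Blueprint for an SSTV station, which by its name is paired with dialogue.
; Entering station range starts a decoder and leaving stops it; a successful decode starts the station and locks it.
; A received mod marker containing "SSTV" finds the BP_SSTV_Printer, spawns the station asset's SSTV class at its spawn position, and triggers a new SDR document on the printer.
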(event EventBeginPlay)

(event Collision|EventActorBeginOverlap
  (params (OtherActor :type Actor%20Object%20Reference)))

(event EventTick
  (params (DeltaSeconds :type Float%20%28single-precision%29)))

(event EventOnDecoded
  (Class|Station|StartStation)
  (Class|Dialogue|Lock true))

(event EventOnEnteringStationRange
  (Class|Station|StartDecoder))

(event EventOnLeavingStationRange
  (Class|Station|StopDecoder))

(event EventOnModMarkerReceived
  (params (Marker :type String))
  (if (Utilities|String|Contains Marker "SSTV")
    (bind _returnvalue (Actor|GetActorOfClass "/Game/03_GPE/SSTV/BP_SSTV_Printer.BP_SSTV_Printer_C"))
    (Utilities|IsValid _returnvalue
      (:Is%20Valid
        (Game|SpawnActorfromClass (Variables|/Script/TheListener.StationAsset|GetSSTVClass (Variables|Default|GetStationAsset)) (Math|Transform|MakeTransform (Transformation|GetWorldLocation (Variables|/Game/03_GPE/SSTV/BP_SSTV_Printer.BP_SSTV_Printer_C|GetSpawnPosition _returnvalue))) "Undefined" "MultiplyWithRoot" 0 0)
        (Default|NewSDRDoc _returnvalue)))))

(fn ConstructionScript)