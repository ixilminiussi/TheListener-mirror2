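; BP_Radio is a possessable radio with a clickable knob and a needle that shows signal clarity.
; Knob clicks play a Wwise sound with haptics: audio-based vibration on DualSense, an attached force feedback effect on other controllers.
; Possession applies DualSense trigger resistance, cleared on unpossess.
; Clarity updates interpolate the needle pivot's rotation, mixed with timer-refreshed random noise to make it jitter.
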(event Custom|NewNoise
  (Variables|Default|SetNoise (Math|Random|RandomFloat)))

(event Custom|OnClick_Event
  (params (IsIncreasing :type Boolean))
  (bind _returnvalue (Game|GetPlayerController 0))
  (bind _returnvalue_2 (Class|GameplayStatics|GetPlayerControllerID _returnvalue))
  (Class|AkGameplayStatics|PostEvent "/Game/WwiseAudio/Events/Default_Work_Unit/radio/play_radio_click.play_radio_click")
  (Utilities|IsValid _returnvalue
    (:Is%20Valid
      (bind _result (CallFunction|IsDualSense _returnvalue_2))
      (if _result
        (if IsIncreasing
          (Class|DualSenseProxy|SetVibrationfromAudio _returnvalue_2 0.0 1.0 50 0.5 0.8 0.015 2.0 1.5)
          (else
            (Class|DualSenseProxy|SetVibrationfromAudio _returnvalue_2 1.0 0.0 50 0.5 0.8 0.015 2.0 1.5)))
        (else
          (ForceFeedback|SpawnForceFeedbackAttached "/Game/03_GPE/Radio/Blueprints/Feedbacks/FFE_ClickRadio.FFE_ClickRadio" (Variables|Default|GetRumbleKnob) "None" "0, 0, 0" "0, 0, 0" "KeepRelativeOffset" false false 1.0 0.0 0))))))

(event EventBeginPlay
  (bind _returnvalue (Game|GetPlayerController 0))
  (bind _knobcomponent (Variables|Default|GetKnobComponent))
  (Utilities|Time|SetTimerbyEvent (delegate Custom|NewNoise) 0.05 true true)
  (bind _asbp_luka_hud (Utilities|Casting|CastToBP_LukaHUD (HUD|GetHUD (Game|GetPlayerController 0))))
  (Variables|Default|SetLuka_HUD _asbp_luka_hud)
  (Utilities|IsValid _knobcomponent
    (:Is%20Valid
      (EventDispatchers|BindEventtoOnClick _knobcomponent (delegate Custom|OnClick_Event))
      (Utilities|IsValid _returnvalue
        (:Is%20Valid
          (bind _result (CallFunction|IsDualSense (Class|GameplayStatics|GetPlayerControllerID _returnvalue)))
          (if (not _result)
            (bind _returnvalue_2 (AddComponent|AddForceFeedbackComponent false (Transformation|GetActorTransform)))
            (Variables|Default|SetRumbleKnob _returnvalue_2)))))))

(event EventOnClarityUpdate
  (params (InClarity :type Float%20%28single-precision%29))
  (bind _clockhandpivotshake (Variables|Default|GetClockHandPivotShake))
  (Transformation|SetRelativeRotation _clockhandpivotshake (Math|Interpolation|RInterpTo (Variables|/Script/Engine.SceneComponent|GetRelativeRotation _clockhandpivotshake) (Math|Rotator|MakeRotator (+ (* (- (* (+ InClarity (* (Variables|Default|GetNoise) 0.5)) 2.0) 1.0) -17.0) 6.0) 0.0 0.0) (Utilities|Time|GetWorldDeltaSeconds) (Variables|ClockHand|GetMovementLerpAlpha)) false false))

(event EventUnpossessed
  (params (OldController :type Controller%20Object%20Reference))
  (bind _returnvalue (Game|GetPlayerController 0))
  (Utilities|IsValid _returnvalue
    (:Is%20Valid
      (bind _result (CallFunction|IsDualSense (Class|GameplayStatics|GetPlayerControllerID _returnvalue)))
      (if _result
        (Class|DualSenseProxy|StopTriggerEffect 0 "AnyHand")))))

(event EventPossessed
  (params (NewController :type Controller%20Object%20Reference))
  (bind _returnvalue (Game|GetPlayerController 0))
  (Utilities|IsValid _returnvalue
    (:Is%20Valid
      (bind _result (CallFunction|IsDualSense (Class|GameplayStatics|GetPlayerControllerID _returnvalue)))
      (if _result
        (Class|DualSenseProxy|SetFeedback 0 2 2 2 "AnyHand")))))

(fn ConstructionScript)

(fn IsDualSense
  (params (ControllerId :type Integer))
  (bind _returnvalue (Class|SonyGamepadProxy|DeviceIsConnected ControllerId))
  (if _returnvalue
    (bind _returnvalue_2 (Class|SonyGamepadProxy|GetDeviceType))
    (return (or (Utilities|Enum|Equal(Enum) _returnvalue_2 "DualSense") (Utilities|Enum|Equal(Enum) _returnvalue_2 "DualSenseEdge")))
    (else
      (return false))))