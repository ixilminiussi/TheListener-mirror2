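; Procedural village house that rebuilds from static mesh components in its construction script, using a random stream seeded by world location.
; It stacks random wall floors to a set or randomised height, adds a random roof and optionally a ground-traced tower.
; Traces from four corner arrows find the terrain drop, which is filled with floors and a bottom piece.
; Floors flip by dot product against BP_Village's DoorsTarget to orient doors.
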(event Custom|house)

(event EventBeginPlay)

(event Collision|EventActorBeginOverlap
  (params (OtherActor :type Actor%20Object%20Reference)))

(event EventTick
  (params (DeltaSeconds :type Float%20%28single-precision%29)))

(fn ConstructionScript
  (Variables|Default|Setskip%20new%20seed%20? true)
  (House|ConstructHouse))

(fn ConstructHouse
  (bind _defaultsceneroot (Variables|Default|GetDefaultSceneRoot))
  (bind _randomised_height_range (Variables|House|Getrandomised%20height%20range))
  (bind _defaultsceneroot_2 (Variables|Default|GetDefaultSceneRoot))
  (bind _returnvalue (Math|Vector|GetForwardVector _defaultsceneroot_2))
  (bind _returnvalue_2 (Transformation|GetWorldLocation _defaultsceneroot))
  (bind _returnvalue_3 (Math|Vector|RotateVectorAroundAxis _returnvalue -9e+01 "0.000000,0.000000,1.000000"))
  (bind (_x _y _z) (Math|Vector|BreakVector _returnvalue_2))
  (bind _returnvalue_4 (Class|KismetMathLibrary|VectorNormal2D _returnvalue_3 0.0001))
  (bind (_x_2 _y_2) (Math|Vector|BreakVector _returnvalue_4))
  (if (Variables|Default|Getskip%20new%20seed%20?)
    (Variables|Default|Setskip%20new%20seed%20? false)
    (else
      (Transformation|AddActorLocalOffset (Math|Vector|MakeVector 0.0 0.0 0.01) false false)))
  (LocalVariables|SetStream (Math|Random|MakeRandomStream (+ (Math|Float|Truncate (+ _x _y)) (Math|Float|Truncate (* _z 1e+02)))))
  (for _array_element (Variables|Default|Getmesh%20ref)
    (Components|DestroyComponent _array_element))
  (Utilities|Array|Clear (Variables|Default|Getfloors%20ref))
  (Utilities|Array|Clear (Variables|Default|Getmesh%20ref))
  (bind _output_get (LocalVariables|Setnumber%20of%20floors (Math|Integer|Clamp(Integer) (Math|Integer|SelectInt (Math|Random|RandomIntegerinRangefromStream (LocalVariables|GetStream) (.x _randomised_height_range) (.y _randomised_height_range)) (Variables|House|GetHouse%20height) (Variables|House|Getrandomise%20height%20?)) 1 100000)))
  (LocalVariables|Setmin%20height 0.0)
  (for _index (range 1 _output_get)
    ;[0.15 0.15 0.15 0.5] build walls
    (switch int (Math|Random|RandomIntegerinRangefromStream (LocalVariables|GetStream) 0 1)
      (:0
        (bind _returnvalue_5 (AddComponent|AddStaticMeshComponent false (Math|Transform|MakeTransform (Math|Vector|MakeVector 0.0 0.0 (* (- _index 1) 2e+02)))))
        (Utilities|Array|Add (Variables|Default|Getmesh%20ref) _returnvalue_5)
        (Utilities|Array|Add (Variables|Default|Getfloors%20ref) _returnvalue_5))
      (:1
        (bind _returnvalue_6 (AddComponent|AddStaticMeshComponent false (Math|Transform|MakeTransform (Math|Vector|MakeVector 0.0 0.0 (* (- _index 1) 2e+02)))))
        (Utilities|Array|Add (Variables|Default|Getmesh%20ref) _returnvalue_6)
        (Utilities|Array|Add (Variables|Default|Getfloors%20ref) _returnvalue_6))))
  (if (Variables|House|Gettower%20?)
    (CallFunction|AddTower))
  ;[0.15 0.15 0.15 0.5] build roof
  (switch int (Math|Random|RandomIntegerinRangefromStream (LocalVariables|GetStream) 0 3)
    (:0
      (bind _returnvalue_7 (AddComponent|AddStaticMeshComponent false (Math|Transform|MakeTransform (Math|Vector|MakeVector 0.0 0.0 (Math|Conversions|ToFloat(Integer) (* (LocalVariables|Getnumber%20of%20floors) 200))))))
      (Utilities|Array|Add (Variables|Default|Getmesh%20ref) _returnvalue_7))
    (:1
      (bind _returnvalue_8 (AddComponent|AddStaticMeshComponent false (Math|Transform|MakeTransform (Math|Vector|MakeVector 0.0 0.0 (Math|Conversions|ToFloat(Integer) (* (LocalVariables|Getnumber%20of%20floors) 200))))))
      (Utilities|Array|Add (Variables|Default|Getmesh%20ref) _returnvalue_8))
    (:2
      (bind _returnvalue_9 (AddComponent|AddStaticMeshComponent false (Math|Transform|MakeTransform (Math|Vector|MakeVector 0.0 0.0 (Math|Conversions|ToFloat(Integer) (* (LocalVariables|Getnumber%20of%20floors) 200))))))
      (Utilities|Array|Add (Variables|Default|Getmesh%20ref) _returnvalue_9))
    (:3
      (bind _returnvalue_10 (AddComponent|AddStaticMeshComponent false (Math|Transform|MakeTransform (Math|Vector|MakeVector 0.0 0.0 (Math|Conversions|ToFloat(Integer) (* (LocalVariables|Getnumber%20of%20floors) 200))))))
      (Utilities|Array|Add (Variables|Default|Getmesh%20ref) _returnvalue_10)))
  ;[0.15 0.15 0.15 0.5] get lowest point
  (for _index_2 (range 0 3)
    (switch int _index_2
      (:0
        (LocalVariables|Settemp%20corner%20loc (Transformation|GetWorldLocation (Variables|Default|GetArrow))))
      (:1
        (LocalVariables|Settemp%20corner%20loc (Transformation|GetWorldLocation (Variables|Default|GetArrow1))))
      (:2
        (LocalVariables|Settemp%20corner%20loc (Transformation|GetWorldLocation (Variables|Default|GetArrow2))))
      (:3
        (LocalVariables|Settemp%20corner%20loc (Transformation|GetWorldLocation (Variables|Default|GetArrow3)))))
    (bind _outhit (Collision|LineTraceByChannel (LocalVariables|Gettemp%20corner%20loc) (- (LocalVariables|Gettemp%20corner%20loc) (Math|Vector|MakeVector 0.0 0.0 1e+03)) "TraceTypeQuery1" false 0 "None"))
    (if (.bBlockingHit (Collision|BreakHitResult _outhit))
      (if (> (- (.z (Transformation|GetWorldLocation (Variables|Default|GetDefaultSceneRoot))) (.Z (Math|Vector|BreakVector (.ImpactPoint (Collision|BreakHitResult _outhit))))) (LocalVariables|Getmin%20height))
        (LocalVariables|Setmin%20height (- (.z (Transformation|GetWorldLocation (Variables|Default|GetDefaultSceneRoot))) (.Z (Math|Vector|BreakVector (.ImpactPoint (Collision|BreakHitResult _outhit)))))))))
  (for _index_3 (range 1 (Math|Integer|Clamp(Integer) (Math|Float|Ceil (/ (LocalVariables|Getmin%20height) 2e+02)) 1 10000))
    (if (== _index_3 (Math|Integer|Clamp(Integer) (Math|Float|Ceil (/ (LocalVariables|Getmin%20height) 2e+02)) 1 10000))
      (bind _returnvalue_11 (AddComponent|AddStaticMeshComponent false (Math|Transform|MakeTransform (Math|Vector|MakeVector 0.0 0.0 (Math|Conversions|ToFloat(Integer) (* _index_3 -200))))))
      (Utilities|Array|Add (Variables|Default|Getmesh%20ref) _returnvalue_11)
      (else
        ;[0.15 0.15 0.15 0.5] build bottom walls
        (switch int (Math|Random|RandomIntegerinRangefromStream (LocalVariables|GetStream) 0 1)
          (:0
            (bind _returnvalue_12 (AddComponent|AddStaticMeshComponent false (Math|Transform|MakeTransform (Math|Vector|MakeVector 0.0 0.0 (Math|Conversions|ToFloat(Integer) (* _index_3 -200))))))
            (Utilities|Array|Add (Variables|Default|Getmesh%20ref) _returnvalue_12)
            (Utilities|Array|Add (Variables|Default|Getfloors%20ref) _returnvalue_12))
          (:1
            (bind _returnvalue_13 (AddComponent|AddStaticMeshComponent false (Math|Transform|MakeTransform (Math|Vector|MakeVector 0.0 0.0 (Math|Conversions|ToFloat(Integer) (* _index_3 -200))))))
            (Utilities|Array|Add (Variables|Default|Getmesh%20ref) _returnvalue_13)
            (Utilities|Array|Add (Variables|Default|Getfloors%20ref) _returnvalue_13))))))
  (bind _returnvalue_14 (Actor|GetActorOfClass "/Game/Village-Tools/02_PCG/02_Blueprints/BP_Village.BP_Village_C"))
  ;[0.15 0.15 0.15 0.5] turn lowest floor
  (if (< (Math|Vector2D|DotProduct(2D) (Math|Vector2D|MakeVector2D _x_2 _y_2) (Math|Vector2D|MakeVector2D (.X (Math|Vector|BreakVector (Class|KismetMathLibrary|VectorNormal2D (- (Transformation|GetWorldLocation (Variables|/Game/Village-Tools/02_PCG/02_Blueprints/BP_Village.BP_Village_C|GetDoors_Target _returnvalue_14)) (Transformation|GetWorldLocation _defaultsceneroot_2)) 0.0001))) (.Y (Math|Vector|BreakVector (Class|KismetMathLibrary|VectorNormal2D (- (Transformation|GetWorldLocation (Variables|/Game/Village-Tools/02_PCG/02_Blueprints/BP_Village.BP_Village_C|GetDoors_Target _returnvalue_14)) (Transformation|GetWorldLocation _defaultsceneroot_2)) 0.0001))))) -0.01)
    (for _array_element_2 (Variables|Default|Getfloors%20ref)
      (Transformation|AddRelativeRotation _array_element_2 "0.000000,180.000000,0.000000" false false))
    (Transformation|AddRelativeRotation (Utilities|Array|Get(acopy) (Variables|Default|Getfloors%20ref)) "0.000000,180.000000,0.000000" false false)
    (else
      (Transformation|AddRelativeRotation (Utilities|Array|Get(acopy) (Variables|Default|Getfloors%20ref)) "0.000000,180.000000,0.000000" false false))))

(fn AddTower
  (bind _arrow (Variables|Default|GetArrow))
  (bind _returnvalue (Transformation|GetWorldLocation _arrow))
  (bind _outhit (Collision|LineTraceByChannel _returnvalue (- _returnvalue (Math|Vector|MakeVector 0.0 0.0 1e+03)) "TraceTypeQuery1" false 0 "ForDuration"))
  (if (.bBlockingHit (Collision|BreakHitResult _outhit))
    (bind _returnvalue_2 (AddComponent|AddStaticMeshComponent false (Math|Transform|MakeTransform (Math|Vector|MakeVector 4e+02 3e+02 (Utilities|Operators|Subtract (.Z (Math|Vector|BreakVector (.ImpactPoint (Collision|BreakHitResult _outhit)))) (.z (Transformation|GetWorldLocation (Variables|Default|GetArrow))) (Variables|House|Gettower%20offset))) "0.000000,-90.000000,0.000000" "1.000000,1.000000,1.000000")))
    (Utilities|Array|Add (Variables|Default|Getmesh%20ref) _returnvalue_2)))