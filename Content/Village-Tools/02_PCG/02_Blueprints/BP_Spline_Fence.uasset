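; Spline-driven village fence tool that builds a weathered wooden-style fence along SplineFence in the construction script.
; CreateFence adds Vertical instanced-mesh posts at scaled DistanceBetweenVertical intervals, aligned to the spline tangent.
; Between neighboring posts it adds two stacked Horizontal rail instances with jittered position and rotation, randomly omitting some by DestructionWeight.
; A random stream seeded from the actor's location keeps the variation deterministic per placement.
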(event EventBeginPlay)

(event Collision|EventActorBeginOverlap
  (params (OtherActor :type Actor%20Object%20Reference)))

(event EventTick
  (params (DeltaSeconds :type Float%20%28single-precision%29)))

(fn ConstructionScript
  (CallFunction|CreateFence))

(fn CreateFence
  (bind _spline_fence (Variables|Default|GetSpline_Fence))
  (LocalVariables|Setdistance%20between%20vertical (* (LocalVariables|Getdistance%20between%20vertical) (.x (Transformation|GetWorldScale (Variables|Default|GetDefaultSceneRoot)))))
  (LocalVariables|Setstream (Math|Random|MakeRandomStreamfromLocation (Transformation|GetWorldLocation (Variables|Default|GetDefaultSceneRoot)) 2e+02 false))
  (for _index (range 0 (Math|Float|Truncate (/ (Spline|GetSplineLength (Variables|Default|GetSpline_Fence)) (LocalVariables|Getdistance%20between%20vertical))))
    (LocalVariables|Setcurrent%20index _index)
    (Components|InstancedStaticMesh|AddInstance (Variables|Default|Getvertical) (Math|Transform|MakeTransform (Spline|GetLocationatDistanceAlongSpline _spline_fence (* (LocalVariables|Getdistance%20between%20vertical) _index) "Local") (Math|Conversions|RotationFromXVector (Spline|GetTangentatDistanceAlongSpline _spline_fence (* (LocalVariables|Getdistance%20between%20vertical) _index) "Local"))) false)
    (if (!= (LocalVariables|Getcurrent%20index) 0)
      (for _index_2 (range 0 1)
        (if (not (Class|KismetMathLibrary|RandomBoolwithWeightfromStream (LocalVariables|Getstream) (Variables|Default|Getdestruction%20weight)))
          (Components|InstancedStaticMesh|AddInstance (Variables|Default|Gethorizontal) (Math|Transform|MakeTransform (+ (+ (Math|Vector|Lerp(Vector) (Spline|GetLocationatDistanceAlongSpline (Variables|Default|GetSpline_Fence) (* (LocalVariables|Getdistance%20between%20vertical) (- (LocalVariables|Getcurrent%20index) 1)) "Local") (Spline|GetLocationatDistanceAlongSpline (Variables|Default|GetSpline_Fence) (* (LocalVariables|Getdistance%20between%20vertical) (LocalVariables|Getcurrent%20index)) "Local") 0.5) (Math|Vector|MakeVector 0.0 0.0 (+ (* _index_2 7e+01) 4e+01))) (Math|Vector|MakeVector 0.0 (Math|Random|RandomFloatinRangefromStream (LocalVariables|Getstream) -5.0 5.0) (Math|Random|RandomFloatinRangefromStream (LocalVariables|Getstream) -1e+01 1e+01))) (Math|Rotator|MakeRotator (+ (.Roll (Math|Rotator|BreakRotator (Math|Rotator|FindLookatRotation (Spline|GetLocationatDistanceAlongSpline (Variables|Default|GetSpline_Fence) (* (LocalVariables|Getdistance%20between%20vertical) (- (LocalVariables|Getcurrent%20index) 1)) "Local") (Spline|GetLocationatDistanceAlongSpline (Variables|Default|GetSpline_Fence) (* (LocalVariables|Getdistance%20between%20vertical) (LocalVariables|Getcurrent%20index)) "Local")))) (Math|Random|RandomFloatinRangefromStream (LocalVariables|Getstream) -5.0 5.0)) (+ (.Pitch (Math|Rotator|BreakRotator (Math|Rotator|FindLookatRotation (Spline|GetLocationatDistanceAlongSpline (Variables|Default|GetSpline_Fence) (* (LocalVariables|Getdistance%20between%20vertical) (- (LocalVariables|Getcurrent%20index) 1)) "Local") (Spline|GetLocationatDistanceAlongSpline (Variables|Default|GetSpline_Fence) (* (LocalVariables|Getdistance%20between%20vertical) (LocalVariables|Getcurrent%20index)) "Local")))) (Math|Random|RandomFloatinRangefromStream (LocalVariables|Getstream) -8.0 8.0)) (+ (.Yaw (Math|Rotator|BreakRotator (Math|Rotator|FindLookatRotation (Spline|GetLocationatDistanceAlongSpline (Variables|Default|GetSpline_Fence) (* (LocalVariables|Getdistance%20between%20vertical) (- (LocalVariables|Getcurrent%20index) 1)) "Local") (Spline|GetLocationatDistanceAlongSpline (Variables|Default|GetSpline_Fence) (* (LocalVariables|Getdistance%20between%20vertical) (LocalVariables|Getcurrent%20index)) "Local")))) (Math|Random|RandomFloatinRangefromStream (LocalVariables|Getstream) -5.0 5.0)))) false))))))