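; Procedural electric pole line that places pole meshes and cables along an editable spline in the construction script.
; Poles sit at fixed distance intervals, aligned to the spline tangent, skipping the first and last sample points.
; Two side-offset cable components link consecutive points at pole-top height, dropping to spline level at both ends of the line.
; Each cable's length is set slightly shorter than its span.
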(fn ConstructionScript
  (CallFunction|CreatePoleSpline))

(fn CreatePoleSpline
  (bind _distance_between_poles (Variables|Default|Getdistance%20between%20poles))
  (bind _spline_pole (Variables|Default|GetSpline_Pole))
  (bind _spline_pole_2 (Variables|Default|GetSpline_Pole))
  (bind _spline_pole_3 (Variables|Default|GetSpline_Pole))
  (bind _returnvalue (Spline|GetSplineLength _spline_pole_2))
  (bind _returnvalue_2 (/ _returnvalue _distance_between_poles))
  (bind _returnvalue_3 (Math|Float|Truncate _returnvalue_2))
  ;[0.15 0.15 0.15 0.5] i'm tired so spagetti it is
  (for _index (range 0 _returnvalue_3)
    (if (or (== _index 0) (== _index _returnvalue_3))
      _
      (else
        (AddComponent|AddStaticMeshComponent false (Math|Transform|MakeTransform (Spline|GetLocationatDistanceAlongSpline _spline_pole (* _index (Variables|Default|Getdistance%20between%20poles)) "Local") (Math|Conversions|RotationFromXVector (Spline|GetTangentatDistanceAlongSpline _spline_pole (* _index (Variables|Default|Getdistance%20between%20poles)) "Local"))))))
    (for _index_2 (range 0 1)
      (if (not (== _index 0))
        (bind _returnvalue_4 (AddComponent|AddCableComponent false (Math|Transform|MakeTransform (+ (+ (.Location (Math|Transform|BreakTransform (Math|Transform|MakeTransform (Spline|GetLocationatDistanceAlongSpline _spline_pole (* _index (Variables|Default|Getdistance%20between%20poles)) "Local") (Math|Conversions|RotationFromXVector (Spline|GetTangentatDistanceAlongSpline _spline_pole (* _index (Variables|Default|Getdistance%20between%20poles)) "Local"))))) (Math|Vector|RotateVectorAroundAxis (Math|Vector|MakeVector -2e+01 (+ 9e+01 (* _index_2 -180)) 0.0) (.Yaw (Math|Rotator|BreakRotator (Math|Conversions|RotationFromXVector (Spline|GetTangentatDistanceAlongSpline _spline_pole (* _index (Variables|Default|Getdistance%20between%20poles)) "Local")))) "0.000000,0.000000,1.000000")) (Math|Vector|MakeVector 0.0 0.0 (Math|Float|SelectFloat 0.0 1.14e+03 (== _index _returnvalue_3)))))))
        (bind _output_get (Variables|/Script/CableComponent.CableComponent|SetEndLocation _returnvalue_4 (+ (+ (Spline|GetLocationatDistanceAlongSpline _spline_pole_3 (* (- _index 1) (Variables|Default|Getdistance%20between%20poles)) "Local") (Math|Vector|RotateVectorAroundAxis (Math|Vector|MakeVector -2e+01 (+ 9e+01 (* _index_2 -180)) 0.0) (.Yaw (Math|Rotator|BreakRotator (Math|Conversions|RotationFromXVector (Spline|GetTangentatDistanceAlongSpline _spline_pole_3 (* (- _index 1) (Variables|Default|Getdistance%20between%20poles)) "Local")))) "0.000000,0.000000,1.000000")) (Math|Vector|MakeVector 0.0 0.0 (Math|Float|SelectFloat 0.0 1.14e+03 (== _index 1))))))
        (Variables|/Script/CableComponent.CableComponent|SetCableLength _returnvalue_4 (* (Math|Vector|Distance(Vector) (+ (+ (.Location (Math|Transform|BreakTransform (Math|Transform|MakeTransform (Spline|GetLocationatDistanceAlongSpline _spline_pole (* _index (Variables|Default|Getdistance%20between%20poles)) "Local") (Math|Conversions|RotationFromXVector (Spline|GetTangentatDistanceAlongSpline _spline_pole (* _index (Variables|Default|Getdistance%20between%20poles)) "Local"))))) (Math|Vector|RotateVectorAroundAxis (Math|Vector|MakeVector -2e+01 (+ 9e+01 (* _index_2 -180)) 0.0) (.Yaw (Math|Rotator|BreakRotator (Math|Conversions|RotationFromXVector (Spline|GetTangentatDistanceAlongSpline _spline_pole (* _index (Variables|Default|Getdistance%20between%20poles)) "Local")))) "0.000000,0.000000,1.000000")) (Math|Vector|MakeVector 0.0 0.0 (Math|Float|SelectFloat 0.0 1.14e+03 (== _index _returnvalue_3)))) _output_get) 0.9))))))