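; Spline-driven stone wall Blueprint that lays wall meshes along an editable spline, capped by left and right pillar pieces.
; The construction script calls generatesplinemesh, which derives segment length from the Mesh variable's X bounds and the piece count from spline length.
; Each segment becomes a shadow-casting, collision-free spline mesh component: pillars at first and last index, long wall between.
; Tangents are clamped to segment length.
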(event Custom|generate%20spline%20mesh
  (bind _spline (Variables|Default|GetSpline))
  (bind _spline_2 (Variables|Default|GetSpline))
  (bind _output_get (Variables|Default|SetLenght (.x (+ (Math|Vector|VectorGetAbs (.min (StaticMesh|GetBoundingBox (Variables|Default|GetMesh)))) (Math|Vector|VectorGetAbs (.max (StaticMesh|GetBoundingBox (Variables|Default|GetMesh))))))))
  (bind _output_get_2 (Variables|Default|Setlast%20index (Math|Float|Truncate (/ (Spline|GetSplineLength (Variables|Default|GetSpline)) _output_get))))
  (for _index (range 0 _output_get_2)
    (if (== _index 0)
      (Variables|Default|SetMesh "/Game/Village-Tools/03_Models/01_Village_Modular_Kit/SM_Piliermur_G.SM_Piliermur_G")
      (elif (== _index _output_get_2)
        (Variables|Default|SetMesh "/Game/Village-Tools/03_Models/01_Village_Modular_Kit/SM_Piliermur_D.SM_Piliermur_D")
        (else
          (Variables|Default|SetMesh "/Game/Village-Tools/03_Models/01_Village_Modular_Kit/SM_mur_long.SM_mur_long"))))
    (bind _returnvalue (AddComponent|AddSplineMeshComponent false))
    (Rendering|SetCastShadow _returnvalue true)
    (Collision|SetCollisionEnabled _returnvalue "NoCollision")
    (SplineMesh|SetForwardAxis _returnvalue "X" true)
    (Components|StaticMesh|SetStaticMesh _returnvalue (Variables|Default|GetMesh))
    (SplineMesh|SetStartandEnd _returnvalue (Spline|GetLocationatDistanceAlongSpline _spline (* _index (Variables|Default|GetLenght)) "Local") (Math|Vector|ClampVectorSize (Spline|GetTangentatDistanceAlongSpline _spline (* _index (Variables|Default|GetLenght)) "Local") 0.0 (Variables|Default|GetLenght)) (Spline|GetLocationatDistanceAlongSpline _spline_2 (* (+ _index 1) (Variables|Default|GetLenght)) "Local") (Math|Vector|ClampVectorSize (Spline|GetTangentatDistanceAlongSpline _spline_2 (* (+ _index 1) (Variables|Default|GetLenght)) "Local") 0.0 (Variables|Default|GetLenght)) true :!class /Script/Engine.SplineMeshComponent)))

(event EventBeginPlay)

(event Collision|EventActorBeginOverlap
  (params (OtherActor :type Actor%20Object%20Reference)))

(event EventTick
  (params (DeltaSeconds :type Float%20%28single-precision%29)))

(fn ConstructionScript
  (CallFunction|GenerateSplineMesh))