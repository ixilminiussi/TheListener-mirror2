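; Game manager for narration custom actions, exposing world-side events for lighting, spawning, interactables, toys, sound, level changes and note notifications.
; Sky events drive Ultra Dynamic Sky time of day, while ManageLights switches or flickers house and city light lists, using a light function for house flicker.
; Other events make Luka pick up the log or speak, toggle 3D sounds by class, unlock phone numbers by name, and async-load levels behind a black screen.
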(event Custom|PickupLog
  (bind _returnvalue (Actor|GetActorOfClass "/Game/09_Props/Interactives/BP_Log.BP_Log_C"))
  (bind _asbp_luka_character (Utilities|Casting|CastToBP_LukaCharacter (Game|GetPlayerCharacter 0)))
  (Utilities|IsValid _returnvalue
    (:Is%20Valid
      (Class|PickupComponent|TryPickup (Variables|/Script/TheListener.LukaCharacter|GetPickupComponent _asbp_luka_character) _returnvalue))))

(event EventBeginPlay
  (bind _returnvalue (Actor|GetActorOfClass "/Game/UltraDynamicSky/Blueprints/Ultra_Dynamic_Sky.Ultra_Dynamic_Sky_C"))
  (Variables|Lighting|SetUltraDynamicSky _returnvalue)
  (bind _returnvalue_2 (Actor|GetActorOfClass "/Game/03_GPE/Radio/Blueprints/BP_Radio.BP_Radio_C"))
  (Variables|GPEAndToys|SetRadio _returnvalue_2))

(event Custom|ChangeAngleCap
  (params (TimeCap :type Float%20%28double-precision%29))
  (Variables|/Game/UltraDynamicSky/Blueprints/Ultra_Dynamic_Sky.Ultra_Dynamic_Sky_C|SetTimeCap (Variables|Lighting|GetUltraDynamicSky) TimeCap))

(event Custom|BeginSunAngle
  (params (TimeOfDay :type Float%20%28double-precision%29) (AnimateTimeOfDay :type Boolean) (SimulateRealSun :type Boolean) (DayAndNightLength :type Float%20%28double-precision%29))
  (bind _ultradynamicsky (Variables|Lighting|GetUltraDynamicSky))
  (Variables|/Game/UltraDynamicSky/Blueprints/Ultra_Dynamic_Sky.Ultra_Dynamic_Sky_C|SetTime%20of%20Day _ultradynamicsky TimeOfDay)
  (Variables|/Game/UltraDynamicSky/Blueprints/Ultra_Dynamic_Sky.Ultra_Dynamic_Sky_C|SetAnimate%20Time%20of%20Day _ultradynamicsky AnimateTimeOfDay)
  (Variables|/Game/UltraDynamicSky/Blueprints/Ultra_Dynamic_Sky.Ultra_Dynamic_Sky_C|SetSimulate%20Real%20Sun _ultradynamicsky SimulateRealSun)
  (Variables|/Game/UltraDynamicSky/Blueprints/Ultra_Dynamic_Sky.Ultra_Dynamic_Sky_C|SetDay%20Length _ultradynamicsky DayAndNightLength)
  (Variables|/Game/UltraDynamicSky/Blueprints/Ultra_Dynamic_Sky.Ultra_Dynamic_Sky_C|SetNight%20Length _ultradynamicsky DayAndNightLength))

(event Custom|ManageLights
  (params (Lights :type E_Lights%20Enum :default "NewEnumerator0") (State :type E_LightState%20Enum :default "NewEnumerator0"))
  (bind _houselights (Variables|Lighting|GetHouseLights))
  (bind _citylights (Variables|Lighting|GetCityLights))
  (switch Utilities|FlowControl|Switch|SwitchonE_Lights Lights
    (:NewEnumerator0
      (switch Utilities|FlowControl|Switch|SwitchonE_LightState State
        (:NewEnumerator0
          (for _array_element _houselights
            (Rendering|SetVisibility (Variables|/Script/Engine.Light|GetLightComponent (Utilities|ResolveSoftReference _array_element)) true false)
            (Rendering|Components|Light|SetLightFunctionMaterial (Variables|/Script/Engine.Light|GetLightComponent (Utilities|ResolveSoftReference _array_element)) 0)))
        (:NewEnumerator1
          (for _array_element_2 _houselights
            (Rendering|SetVisibility (Variables|/Script/Engine.Light|GetLightComponent (Utilities|ResolveSoftReference _array_element_2)) false false)
            (Rendering|Components|Light|SetLightFunctionMaterial (Variables|/Script/Engine.Light|GetLightComponent (Utilities|ResolveSoftReference _array_element_2)) 0)))
        (:NewEnumerator2
          (for _array_element_3 _houselights
            (Rendering|Components|Light|SetLightFunctionMaterial (Variables|/Script/Engine.Light|GetLightComponent (Utilities|ResolveSoftReference _array_element_3)) "/Game/05_Environment/Inside/Materials/LF_Flicker_Intro.LF_Flicker_Intro")))))
    (:NewEnumerator1
      (switch Utilities|FlowControl|Switch|SwitchonE_LightState State
        (:NewEnumerator0
          (for _array_element_4 _citylights
            (Default|ActivateCityLights (Utilities|ResolveSoftReference _array_element_4))))
        (:NewEnumerator1
          (for _array_element_5 _citylights
            (Default|DeactivateCityLights (Utilities|ResolveSoftReference _array_element_5))))
        (:NewEnumerator2
          (for _array_element_6 _citylights
            (Default|FlickerLight (Utilities|ResolveSoftReference _array_element_6))))))))

(event Custom|SpawnObject
  (params (ObjectToSpawn :type Actor%20Object%20Reference) (SpawnTransform :type Transform))
  (Game|SpawnActorfromClass (Utilities|GetClass ObjectToSpawn) SpawnTransform "Undefined" "MultiplyWithRoot" 0 0))

(event Custom|ManageInteraction
  (params (Interactable :type Interactable%20Soft%20Object%20Reference) (State :type Boolean))
  (Class|Interactable|Enable (Utilities|ResolveSoftReference Interactable) State))

(event Custom|ManageToy
  (params (Toy :type Toy%20Soft%20Object%20Reference) (State :type Boolean))
  (Class|Toy|Enable (Utilities|ResolveSoftReference Toy) State))

(event Custom|ChangeLevel
  (params (LevelToLoad :type Soft%20World%20Reference%20Structure))
  (bind _worldasset (Utilities|Struct|BreakSoftWorldReference LevelToLoad))
  (Utilities|AsyncLoadAsset _worldasset
    (:then
      (bind _returnvalue (UserInterface|CreateWidget "/Game/07_UI/Menus/MainMenu/WBP_BlackScreen.WBP_BlackScreen_C"))
      (UserInterface|Viewport|AddtoViewport _returnvalue 0)
      (Class|EventSubsystem|PauseTimers (Subsystems|GetEventSubsystem)))
    (:Completed
      (Game|OpenLevel(byObjectReference) _worldasset))))

(event Custom|LukaSpeak
  (params (LukaController :type Luka%20Controller%20Object%20Reference) (SoundToPlay :type Ak%20Audio%20Event%20Object%20Reference))
  (bind _asbp_luka_character (Utilities|Casting|CastToBP_LukaCharacter (Class|LukaController|GetLukaCharacter LukaController)))
  (Default|Speak _asbp_luka_character SoundToPlay))

(event Custom|PlaySound3D
  (params (3DSoundToAccess :type BP%203D%20Sound%20Class%20Reference) (Stop? :type Boolean))
  (bind _outactors (Actor|GetAllActorsOfClass 3DSoundToAccess))
  (if Stop?
    (for _array_element _outactors
      (bind _asbp_3dsound (Utilities|Casting|CastToBP_3DSound _array_element))
      (Default|StopSound _asbp_3dsound))
    (else
      (for _array_element_2 _outactors
        (bind _asbp_3dsound_2 (Utilities|Casting|CastToBP_3DSound _array_element_2))
        (Default|PlaySound _asbp_3dsound_2)))))

(event Custom|PlayNotifPhoneCorkboard
  (params (IsCorkboard? :type Boolean) (NoteName :type String))
  (bind _foundwidgets (Widget|GetAllWidgetsOfClass "/Game/07_UI/InGame/WBP_Play.WBP_Play_C" true))
  (for _array_element _foundwidgets
    (Default|NotifNotePhone _array_element IsCorkboard?))
  (bind _returnvalue (Actor|GetActorOfClass "/Game/03_GPE/Phone/Blueprints/BP_Phone.BP_Phone_C"))
  (for _array_element_2 (Class|PanelWidget|GetAllChildren (Variables|/Game/07_UI/Phone/W_PhoneDirectoryTest.W_PhoneDirectoryTest_C|GetNumbers (Variables|/Game/03_GPE/Phone/Blueprints/BP_Phone.BP_Phone_C|GetPhoneDirectory _returnvalue)))
    (if (Utilities|Enum|Equal(Enum) (Utilities|GetObjectName _array_element_2) NoteName)
      (bind _asw_phone_number (Utilities|Casting|CastToW_PhoneNumber _array_element_2))
      (Default|Unlock _asw_phone_number))))

(fn ConstructionScript)